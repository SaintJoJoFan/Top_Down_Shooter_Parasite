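; BP_Wall is a wall piece actor whose appearance is set by its WallType.
; The construction script gives the Wall mesh a tiled side material, then picks the top material by type: inner corner, outer corner, side or single, with the last two sharing one material.
; The Black type overrides both slots with an unlit black material.
; The event graph contains no active logic.
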(fn `UserConstructionScript`
  (`PrimitiveComponent.SetMaterial` (`self.Wall`) 0 "/Game/Models/M_Wall_Side_Tile.M_Wall_Side_Tile")
  (switch `/Game/Models/Wall_Type` (`self.Wall Type`)
    (:`NewEnumerator0`
      (`PrimitiveComponent.SetMaterial` (`self.Wall`) 1 "/Game/Models/M_Wall_Up_Corner_Inner.M_Wall_Up_Corner_Inner"))
    (:`NewEnumerator1`
      (`PrimitiveComponent.SetMaterial` (`self.Wall`) 1 "/Game/Models/M_Wall_Up_Corner_Outer.M_Wall_Up_Corner_Outer"))
    (:`NewEnumerator2`
      (`PrimitiveComponent.SetMaterial` (`self.Wall`) 1 "/Game/Models/M_Wall_Up_Black_Unlit.M_Wall_Up_Black_Unlit")
      (`PrimitiveComponent.SetMaterial` (`self.Wall`) 0 "/Game/Models/M_Wall_Up_Black_Unlit.M_Wall_Up_Black_Unlit"))
    (:`NewEnumerator3`
      (`PrimitiveComponent.SetMaterial` (`self.Wall`) 1 "/Game/Models/M_Wall_Up_Side.M_Wall_Up_Side"))
    (:`NewEnumerator4`
      (`PrimitiveComponent.SetMaterial` (`self.Wall`) 1 "/Game/Models/M_Wall_Up_Side.M_Wall_Up_Side"))))