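; Red-sprited melee cultist character that fights under either player or AI control, with walk and bullet speeds set on possession.
; Left mouse triggers a rate-limited melee box trace that damages opposing pawns or breaks vents.
; Player hits also write the attacker into the victim's AI blackboard as its seen target.
; Attacks alternate scythe swings through stepped RInterpTo rotations, while Tick feeds directional flipbooks to AnimationMachine.
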(event `Melee_Attack`
  (params (Damage :type "Float (double-precision)"))
  (bind _returnvalue (`GameplayStatics.GetWorldDeltaSeconds`))
  (bind _sythe_arrow (`self.Sythe_Arrow`))
  (bind _arrow_gun (`self.Arrow_Gun`))
  (bind _melee_attack_pause (`self.Melee_Attack_Pause`))
  (bind (_returnvalue_location _returnvalue_rotation) (`KismetMathLibrary.BreakTransform` (`SceneComponent.GetRelativeTransform` _sythe_arrow)))
  (bind _returnvalue_2 (`SceneComponent.K2_GetComponentLocation` _arrow_gun))
  (bind _returnvalue_3 (`KismetMathLibrary.RInterpTo` _returnvalue_rotation (struct :`Pitch` 90.0) _returnvalue 10.0))
  (bind _returnvalue_4 (`KismetMathLibrary.RInterpTo` _returnvalue_rotation (struct :`Pitch` -90.0) _returnvalue 10.0))
  ;[1 1 1] Melee Attack
  (`|ExecutionSequence`
    (:`then_0`
      (bind _outhit (`KismetSystemLibrary.BoxTraceSingle` _returnvalue_2 (+ _returnvalue_2 (* (`SceneComponent.GetForwardVector` _arrow_gun) 100.0)) (30.0 30.0 10.0) (struct) "TraceTypeQuery2" false (`|MakeArray` self :!type "Actor Object Reference")))
      (bind (_bblockinghit _binitialoverlap _time _distance _location _impactpoint _normal _impactnormal _physmat _hitactor) (`GameplayStatics.BreakHitResult` _outhit))
      (bind _aspawn (cast `Pawn` _hitactor)
        (:`then`
          (cast `/Game/Blueprints/BP_PlayerController` (`self.GetController`)
            (:`then`
              (bind _returnvalue_5 (`self.GetController` _aspawn))
              (bind _asbp_enemy_controller (cast `/Game/Blueprints/BP_Enemy_Controller` _returnvalue_5))
              (bind _asbp_characters_parent (cast `/Game/Blueprints/BP_Characters_Parent` _aspawn))
              (bind _returnvalue_6 (`AIBlueprintHelperLibrary.GetBlackboard` _asbp_enemy_controller))
              (`BlackboardComponent.SetValueAsObject` _returnvalue_6 "FollowTarget" self)
              (`BlackboardComponent.SetValueAsBool` _returnvalue_6 "Can See?" true)
              (`BlackboardComponent.SetValueAsVector` (`AIBlueprintHelperLibrary.GetBlackboard` _asbp_enemy_controller) "Target_Position" (`self.K2_GetActorLocation` self))
              (`GameplayStatics.ApplyDamage` _asbp_characters_parent Damage))
            (:`CastFailed`
              (cast `/Game/Blueprints/BP_PlayerController` _returnvalue_5)
              (bind _asbp_characters_parent_2 (cast `/Game/Blueprints/BP_Characters_Parent` _aspawn))
              (`GameplayStatics.ApplyDamage` _asbp_characters_parent_2 Damage)))
          (`GameplayStatics.PlaySound2D` "/Game/Sounds/SND_Slash.SND_Slash" 1.0 1.0 0.0 null null))
        (:`CastFailed`
          (bind _asbp_vent (cast `/Game/Blueprints/BP_Vent` _hitactor))
          (`GameplayStatics.PlaySound2D` "/Game/Sounds/SND_Vent_Break.SND_Vent_Break" 1.0 1.0 0.0 null null)
          (`self.K2_DestroyActor` _asbp_vent))))
    (:`then_1`
      (`/Engine/EditorBlueprintResources/StandardMacros.FlipFlop`
        (:`A`
          (`SceneComponent.K2_SetRelativeRotation` _sythe_arrow _returnvalue_3 false false)
          (`KismetSystemLibrary.Delay` _melee_attack_pause)
          (`SceneComponent.K2_SetRelativeRotation` _sythe_arrow _returnvalue_3 false false)
          (`KismetSystemLibrary.Delay` _melee_attack_pause)
          (`SceneComponent.K2_SetRelativeRotation` _sythe_arrow _returnvalue_3 false false)
          (`KismetSystemLibrary.Delay` _melee_attack_pause)
          (`SceneComponent.K2_SetRelativeRotation` _sythe_arrow _returnvalue_3 false false)
          (`KismetSystemLibrary.Delay` _melee_attack_pause)
          (`SceneComponent.K2_SetRelativeRotation` _sythe_arrow _returnvalue_3 false false))
        (:`B`
          (`SceneComponent.K2_SetRelativeRotation` _sythe_arrow _returnvalue_4 false false)
          (`KismetSystemLibrary.Delay` _melee_attack_pause)
          (`SceneComponent.K2_SetRelativeRotation` _sythe_arrow _returnvalue_4 false false)
          (`KismetSystemLibrary.Delay` _melee_attack_pause)
          (`SceneComponent.K2_SetRelativeRotation` _sythe_arrow _returnvalue_4 false false)
          (`KismetSystemLibrary.Delay` _melee_attack_pause)
          (`SceneComponent.K2_SetRelativeRotation` _sythe_arrow _returnvalue_4 false false)
          (`KismetSystemLibrary.Delay` _melee_attack_pause)
          (`SceneComponent.K2_SetRelativeRotation` _sythe_arrow _returnvalue_4 false false))))))

(event `self.ReceiveUnpossessed`
  (params (OldController :type "Controller Object Reference"))
  (`parent.ReceiveUnpossessed` OldController))

(event `self.ReceivePossessed`
  (params (NewController :type "Controller Object Reference"))
  (`parent.ReceivePossessed` NewController)
  (cast `/Game/Blueprints/BP_PlayerController` NewController
    (:`then`
      (set `CharacterMovementComponent.MaxWalkSpeed` 400.0 (`self.CharacterMovement`))
      (set `self.Bullet_Speed` 700.0))
    (:`CastFailed`
      (cast `/Game/Blueprints/BP_Enemy_Controller` NewController)
      (set `CharacterMovementComponent.MaxWalkSpeed` 350.0 (`self.CharacterMovement`))
      (set `self.Bullet_Speed` 300.0))))

(event `self.ReceiveBeginPlay`
  (`parent.ReceiveBeginPlay`)
  (set `self.Idle_Flipbook` "/Game/Flipbooks/FB_Red_Idle_Down.FB_Red_Idle_Down")
  (bind _output_get (set `self.Health` 14.0))
  (set `self.Health_Max` _output_get))

(event `self.ReceiveTick`
  (params (DeltaSeconds :type "Float (single-precision)"))
  (`parent.ReceiveTick` DeltaSeconds)
  (`self.Animation_Machine` (`self.Sprite`) "/Game/Flipbooks/FB_Red_Walk_Right.FB_Red_Walk_Right" "/Game/Flipbooks/FB_Red_Walk_Down.FB_Red_Walk_Down" "/Game/Flipbooks/FB_Red_Walk_Up.FB_Red_Walk_Up" (`self.Arrow_Bullet`) (`self.Arrow_Gun`) (`self.Gun_FlipBook`) "/Game/Flipbooks/FB_Red_Idle_Right.FB_Red_Idle_Right" "/Game/Flipbooks/FB_Red_Idle_Down.FB_Red_Idle_Down" "/Game/Flipbooks/FB_Red_Idle_Up.FB_Red_Idle_Up" (`self.Arrow_Sprite_Gun`) (`self.Arrow_All_Sprites`)))

(event `EnhancedInput|/Game/Inputs/IA_LeftMouse`
  (params (ActionValue :type Boolean) (ElapsedSeconds :type "Float (double-precision)") (TriggeredSeconds :type "Float (double-precision)") (InputAction :type "InputAction Object Reference" :default "/Game/Inputs/IA_LeftMouse.IA_LeftMouse"))
  (:`Triggered`
    (`/Engine/EditorBlueprintResources/StandardMacros.DoOnce` false :!label _label
      (:`Completed`
        (`self.Melee_Attack` 3.0)
        (`KismetSystemLibrary.Delay` 0.3)
        (goto _label :!via `Reset`)))))

(fn `UserConstructionScript`
  (`parent.UserConstructionScript`))