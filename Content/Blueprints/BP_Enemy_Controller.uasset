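; AI controller for cultist enemies that runs BT_Enemy and flags the possessed cultist type (Mage, Acolyte, Fanatic or Sniper) on the blackboard.
; AI perception writes noise, sight and follow-target keys for player-controlled pawns, treating a parasite under a table as lost from sight.
; A sniper check bypasses the short distance limit otherwise applied to stimuli.
; Tick mirrors the player's pause state and updates the target's position.
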(event `self.ReceivePossess`
  (params (PossessedPawn :type "Pawn Object Reference"))
  (`self.RunBehaviorTree` "/Game/Behavior_Tree/BT_Enemy.BT_Enemy")
  (cast `/Game/Blueprints/BP_Cultist_Mage` PossessedPawn
    (:`then`
      (`BlackboardComponent.SetValueAsBool` (`AIBlueprintHelperLibrary.GetBlackboard` null) "is Mage?" true))
    (:`CastFailed`
      (cast `/Game/Blueprints/BP_Cultist_Acolyte` PossessedPawn
        (:`then`
          (`BlackboardComponent.SetValueAsBool` (`AIBlueprintHelperLibrary.GetBlackboard` null) "is Acolyte?" true))
        (:`CastFailed`
          (cast `/Game/Blueprints/BP_Cultist_Fanatic` PossessedPawn
            (:`then`
              (`BlackboardComponent.SetValueAsBool` (`AIBlueprintHelperLibrary.GetBlackboard` null) "is Fanatic?" true))
            (:`CastFailed`
              (cast `/Game/Blueprints/BP_Cultist_Sniper` PossessedPawn)
              (`BlackboardComponent.SetValueAsBool` (`AIBlueprintHelperLibrary.GetBlackboard` null) "is Sniper?" true))))))))

(event `self.AIPerception.OnTargetPerceptionUpdated`
  (params (Actor :type "Actor Object Reference") (Stimulus :type "AIStimulus Structure"))
  (bind (_age _expirationage _strength _stimuluslocation _receiverlocation _tag _bsuccessfullysensed) (break `AIStimulus` Stimulus))
  (bind (_age_2 _expirationage_2 _strength_2 _stimuluslocation_2 _receiverlocation_2) (break `AIStimulus` Stimulus))
  (if (== (`self.K2_GetPawn`) "/Game/Blueprints/BP_Cultist_Sniper.BP_Cultist_Sniper")
    (bind _aspawn (cast `Pawn` Actor :!label _label))
    (cast `/Game/Blueprints/BP_PlayerController` (`Pawn.GetController` _aspawn))
    (bind _output_get (set `self.Target Actor` Actor))
    (if (== _tag "noise")
      ;[1 1 1] set noise position
      (if _bsuccessfullysensed
        (`BlackboardComponent.SetValueAsVector` (`AIBlueprintHelperLibrary.GetBlackboard` null) "Noise_Position" _stimuluslocation)
        (else
          (`BlackboardComponent.ClearValue` (`AIBlueprintHelperLibrary.GetBlackboard` null) "Noise_Position")))
      (elif _bsuccessfullysensed
        ;[1 1 1] set can see and actor target
        (bind _asbp_parasite (cast `/Game/Blueprints/BP_Parasite` (`self.Target Actor`))
          (:`then`
            (if (not (`/Game/Blueprints/BP_Parasite.Under Table` _asbp_parasite))
              (`BlackboardComponent.SetValueAsBool` (`AIBlueprintHelperLibrary.GetBlackboard` null) "Can See?" true :!label _label_2)
              (`BlackboardComponent.SetValueAsObject` (`AIBlueprintHelperLibrary.GetBlackboard` null) "FollowTarget" _output_get)
              (else
                ;[1 1 1] set can't see and last seen position
                (`BlackboardComponent.ClearValue` (`AIBlueprintHelperLibrary.GetBlackboard` null) "Can See?" :!label _label_3)
                (`BlackboardComponent.ClearValue` (`AIBlueprintHelperLibrary.GetBlackboard` null) "FollowTarget")
                (`BlackboardComponent.SetValueAsVector` (`AIBlueprintHelperLibrary.GetBlackboard` null) "Noise_Position" _stimuluslocation)
                (set `self.Target Actor` null))))
          (:`CastFailed`
            (goto _label_2)))
        (else
          (goto _label_3))))
    (elif (<= (`KismetMathLibrary.Vector_Distance` _stimuluslocation_2 _receiverlocation_2) 350.0)
      (goto _label))))

(event `self.ReceiveTick`
  (params (DeltaSeconds :type "Float (single-precision)"))
  (bind _target_actor (`self.Target Actor`))
  (`BlackboardComponent.SetValueAsBool` (`AIBlueprintHelperLibrary.GetBlackboard` null) "is Paused?" (`/Game/Blueprints/BP_PlayerController.Paused?` (cast `/Game/Blueprints/BP_PlayerController` (`GameplayStatics.GetPlayerController` 0) :!pure true)))
  (`/Engine/EditorBlueprintResources/StandardMacros.IsValid` _target_actor
    (:`Is Valid`
      (`BlackboardComponent.SetValueAsVector` (`AIBlueprintHelperLibrary.GetBlackboard` null) "Target_Position" (`self.K2_GetActorLocation` _target_actor)))))

(fn `UserConstructionScript`)