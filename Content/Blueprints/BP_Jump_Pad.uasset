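; BP_Jump_Pad is a jump pad trigger that bounces the player character, BP_PL_Hacker, upward on overlap.
; The overlap launches the character with a fixed vertical velocity that overrides its current Z speed.
; It also plays the squick flipbook on FollowTarget's sprite, restoring the idle flipbook after one flipbook length.
; Every tick, the pad snaps to just above FollowTarget's location, so it follows that platform actor.
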(event `self.ReceiveActorBeginOverlap`
  (params (OtherActor :type "Actor Object Reference"))
  (bind _sprite (`PaperCharacter.Sprite` (`self.Follow_Target`)))
  (bind _asbp_pl_hacker (cast `/Game/Blueprints/BP_PL_Hacker` OtherActor))
  (`Character.LaunchCharacter` _asbp_pl_hacker (* (`KismetMathLibrary.Vector_Up`) 400.0) false true)
  (`PaperFlipbookComponent.SetFlipbook` _sprite "/Game/Assets/FB_Platform_Squick.FB_Platform_Squick")
  (`KismetSystemLibrary.Delay` (`PaperFlipbookComponent.GetFlipbookLength` _sprite))
  (`PaperFlipbookComponent.SetFlipbook` _sprite "/Game/Assets/FB_Platform_Idle.FB_Platform_Idle"))

(event `self.ReceiveTick`
  (params (DeltaSeconds :type "Float (single-precision)"))
  (bind (_returnvalue_x _returnvalue_y _returnvalue_z) (`KismetMathLibrary.BreakVector` (`self.K2_GetActorLocation` (`self.Follow_Target`))))
  (`self.K2_SetActorLocation` (`KismetMathLibrary.MakeVector` _returnvalue_x _returnvalue_y (+ _returnvalue_z 8.0))))

(fn `UserConstructionScript`)