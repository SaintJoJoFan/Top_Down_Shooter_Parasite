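; Player camera manager that gives BP_Characters_Parent view targets a fixed-rotation, top-down camera with a constant field of view.
; BlueprintUpdateCamera casts the target and interpolates toward a point above the character.
; The interpolation starts from the character's location each frame rather than the previous camera location, so the height offset depends on frame time and motion is not smoothed.
; An ArrowGun-based position calculation is left unused.
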(fn `BlueprintUpdateCamera`
  (params (CameraTarget :type "Actor Object Reference"))
  (returns (NewCameraLocation :type "Vector Structure") (NewCameraRotation :type "Rotator Structure") (NewCameraFOV :type "Float (single-precision)") (ReturnValue :type Boolean))
  (bind _asbp_characters_parent (cast `/Game/Blueprints/BP_Characters_Parent` CameraTarget))
  (bind (_returnvalue_x _returnvalue_y _returnvalue_z) (`KismetMathLibrary.BreakVector` (`self.K2_GetActorLocation` _asbp_characters_parent)))
  (return (`KismetMathLibrary.VInterpTo` (`self.K2_GetActorLocation` _asbp_characters_parent) (`KismetMathLibrary.MakeVector` _returnvalue_x _returnvalue_y (+ _returnvalue_z 300.0)) (`GameplayStatics.GetWorldDeltaSeconds`) 5.0) (struct :`Pitch` 270.0 :`Yaw` -90.0) 90.0 true))

(fn `UserConstructionScript`)