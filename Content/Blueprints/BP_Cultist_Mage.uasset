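; Cultist Mage character that either a player or an enemy controller can possess, with walk and bullet speeds set higher for the player.
; On BeginPlay it sets health and idle flipbook, then each Tick feeds cyan directional flipbooks and shotgun animations into AnimationMachine.
; Left mouse fires one shotgun shot per press unless reloading, starting a reload with sound when bullets run out.
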(event `self.ReceiveBeginPlay`
  (`parent.ReceiveBeginPlay`)
  (set `self.Idle_Flipbook` "/Game/Flipbooks/FB_Cultists/FB_Magos/FB_Cyan_Idle_Down.FB_Cyan_Idle_Down")
  (bind _output_get (set `self.Health` 5.0))
  (set `self.Health_Max` _output_get))

(event `self.ReceiveUnpossessed`
  (params (OldController :type "Controller Object Reference"))
  (`parent.ReceiveUnpossessed` OldController))

(event `self.ReceivePossessed`
  (params (NewController :type "Controller Object Reference"))
  (`parent.ReceivePossessed` NewController)
  (cast `/Game/Blueprints/BP_PlayerController` NewController
    (:`then`
      (set `CharacterMovementComponent.MaxWalkSpeed` 250.0 (`self.CharacterMovement`))
      (set `self.Bullet_Speed` 700.0))
    (:`CastFailed`
      (cast `/Game/Blueprints/BP_Enemy_Controller` NewController)
      (set `CharacterMovementComponent.MaxWalkSpeed` 200.0 (`self.CharacterMovement`))
      (set `self.Bullet_Speed` 300.0))))

(event `self.ReceiveTick`
  (params (DeltaSeconds :type "Float (single-precision)"))
  (`parent.ReceiveTick` DeltaSeconds)
  (`self.Animation Machine` (`self.Sprite`) "/Game/Flipbooks/FB_Cultists/FB_Magos/FB_Cyan_Walk_Right.FB_Cyan_Walk_Right" "/Game/Flipbooks/FB_Cultists/FB_Magos/FB_Cyan_Walk_Left.FB_Cyan_Walk_Left" "/Game/Flipbooks/FB_Cultists/FB_Magos/FB_Cyan_Walk_Down.FB_Cyan_Walk_Down" "/Game/Flipbooks/FB_Cultists/FB_Magos/FB_Cyan_Walk_Up.FB_Cyan_Walk_Up" (`self.Arrow_Bullet`) (`self.Arrow_Gun`) (`self.Gun_FlipBook`) "/Game/Flipbooks/FB_Cultists/FB_Magos/FB_Cyan_Idle_Right.FB_Cyan_Idle_Right" "/Game/Flipbooks/FB_Cultists/FB_Magos/FB_Cyan_Idle_Left.FB_Cyan_Idle_Left" "/Game/Flipbooks/FB_Cultists/FB_Magos/FB_Cyan_Idle_Down.FB_Cyan_Idle_Down" "/Game/Flipbooks/FB_Cultists/FB_Magos/FB_Cyan_Idle_Up.FB_Cyan_Idle_Up" (`self.Arrow_Sprite_Gun`) (`self.Arrow_Root`) (`self.isReloading?`) "/Game/Flipbooks/FB_Weapon/FB_Shotgun_Idle.FB_Shotgun_Idle" "/Game/Flipbooks/FB_Weapon/FB_Shotgun_Reload.FB_Shotgun_Reload"))

(event `EnhancedInput|/Game/Inputs/IA_LeftMouse`
  (params (ActionValue :type Boolean) (ElapsedSeconds :type "Float (double-precision)") (TriggeredSeconds :type "Float (double-precision)") (InputAction :type "InputAction Object Reference" :default "/Game/Inputs/IA_LeftMouse.IA_LeftMouse"))
  (:`Triggered`
    (`/Engine/EditorBlueprintResources/StandardMacros.DoOnce` false :!label _label
      (:`Completed`
        (if (not (`self.isReloading?`))
          (`/Engine/EditorBlueprintResources/StandardMacros.DecrementInt` (`self.Bullets`)
            (:`  `
              (`self.Shoot Shotgun`)
              (if (<= (`self.Bullets`) 0)
                (set `self.isReloading?` true)
                (set `self.Reload_Time` 0.0)
                (`GameplayStatics.PlaySound2D` "/Game/Sounds/Weapon/Reload/Shotgun_Reload.Shotgun_Reload" 1.0 1.0 0.0 null null))))))))
  (:`Completed`
    (goto _label :!via `Reset`)))

(fn `UserConstructionScript`
  (`parent.UserConstructionScript`))