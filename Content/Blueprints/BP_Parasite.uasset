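; BP_Parasite is the player-controllable parasite character, a Paper2D flipbook child of a parent class.
; On possession it sets movement and bullet speeds and loads health from BP_PlayerController; on unpossession it saves health back and destroys itself.
; Each tick it locks the sprite's rotation, picks a directional crawl flipbook from the dominant velocity axis, and stops playback when nearly still.
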(event `self.ReceivePossessed`
  (params (NewController :type "Controller Object Reference"))
  (bind _asbp_player_controller (cast `/Game/Blueprints/BP_PlayerController` NewController))
  (set `CharacterMovementComponent.MaxWalkSpeed` 350.0 (`self.CharacterMovement`))
  (set `self.Bullet_Speed` 500.0)
  (set `self.Health` (`/Game/Blueprints/BP_PlayerController.Parasite_Health` _asbp_player_controller))
  (`self.K2_SetActorRotation` (struct :`Roll` 270.0)))

(event `self.ReceiveUnpossessed`
  (params (OldController :type "Controller Object Reference"))
  (bind _asbp_player_controller (cast `/Game/Blueprints/BP_PlayerController` OldController))
  (set `/Game/Blueprints/BP_PlayerController.Parasite_Health` (`self.Health`) _asbp_player_controller)
  (`self.K2_DestroyActor`))

(event `self.ReceiveBeginPlay`
  (`parent.ReceiveBeginPlay`)
  (set `self.Idle_Flipbook` "/Game/Flipbooks/FB_Crawl_Idle.FB_Crawl_Idle"))

(event `self.ReceiveTick`
  (params (DeltaSeconds :type "Float (single-precision)"))
  (`parent.ReceiveTick` DeltaSeconds)
  (`self.Animation_Parasite` (`self.Sprite`)))

(fn `Animation_Parasite`
  (params (Parasite_Flipbook :type "PaperFlipbookComponent Object Reference"))
  (bind (_returnvalue_x _returnvalue_y) (`KismetMathLibrary.BreakVector` (`self.GetVelocity`)))
  (`|ExecutionSequence`
    (:`then_0`
      (`SceneComponent.K2_SetWorldRotation` Parasite_Flipbook (struct :`Roll` 270.0) false false))
    (:`then_1`
      (if (< (`KismetMathLibrary.VSize` (`self.GetVelocity`)) 3.0)
        (`PaperFlipbookComponent.Stop` Parasite_Flipbook)
        (else
          (`PaperFlipbookComponent.Play` Parasite_Flipbook)
          (if (> (`KismetMathLibrary.Abs` _returnvalue_x) (`KismetMathLibrary.Abs` _returnvalue_y))
            (if (> _returnvalue_x 0.0)
              (`PaperFlipbookComponent.SetFlipbook` Parasite_Flipbook "/Game/Flipbooks/FB_Crawl_Right.FB_Crawl_Right")
              (else
                (`PaperFlipbookComponent.SetFlipbook` Parasite_Flipbook "/Game/Flipbooks/FB_Crawl_Left.FB_Crawl_Left")))
            (elif (> _returnvalue_y 0.0)
              (`PaperFlipbookComponent.SetFlipbook` Parasite_Flipbook "/Game/Flipbooks/FB_Crawl_Down.FB_Crawl_Down")
              (else
                (`PaperFlipbookComponent.SetFlipbook` Parasite_Flipbook "/Game/Flipbooks/FB_Crawl_Up.FB_Crawl_Up")))))))))

(fn `UserConstructionScript`
  (`parent.UserConstructionScript`))