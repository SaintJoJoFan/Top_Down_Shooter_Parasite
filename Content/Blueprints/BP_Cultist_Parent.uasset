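; Parent Blueprint for cultist enemies that the player's parasite can possess and control.
; Under AI control it runs a line-of-sight trace and mesh, which stop on player possession as health drops and the parasite gets a one-time heal if low.
; While possessed, health drains until death, and the action input ejects a new parasite, killing the host.
; Player unpossession returns the AI controller with a temporary blackboard stun.
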(event `self.ReceivePossessed`
  (params (NewController :type "Controller Object Reference"))
  (bind _health (`self.Health`))
  (bind _lineofsight (`self.LineOfSight`))
  (bind _lineofsight_2 (`self.LineOfSight`))
  (bind _asbp_player_controller (cast `/Game/Blueprints/BP_PlayerController` NewController)
    (:`then`
      (`PaperFlipbookComponent.SetFlipbook` (`self.State_Flipbook`) null)
      (`PaperFlipbookComponent.SetFlipbook` (`self.Parasite_Flipbook`) "/Game/Flipbooks/FB_Crawl_Idle.FB_Crawl_Idle")
      (`self.K2_SetActorRotation` (struct :`Roll` 270.0))
      (`LineOfSightComponent.StopLineTrace` _lineofsight_2)
      (`LineOfSightComponent.StopBuildMesh` _lineofsight_2)
      (`|ExecutionSequence`
        (:`then_0`
          (if (> _health 10)
            (set `self.Health` (- _health 6))
            (set `self.Health_Max` (- (`self.Health_Max`) 6))))
        (:`then_1`
          (bind _parasite_health (`/Game/Blueprints/BP_PlayerController.Parasite_Health` _asbp_player_controller))
          (if (and (<= _parasite_health 10.0) (not (`self.Was_Beaten?`)))
            (set `/Game/Blueprints/BP_PlayerController.Parasite_Health` (+ _parasite_health 2.0) _asbp_player_controller)
            (set `self.Was_Beaten?` true)))
        (:`then_2`
          (set `PlayerController.CurrentMouseCursor` "Crosshairs" (`GameplayStatics.GetPlayerController` 0)))))
    (:`CastFailed`
      (bind _asbp_enemy_controller (cast `/Game/Blueprints/BP_Enemy_Controller` NewController))
      (set `self.AI_Controller` _asbp_enemy_controller)
      (`LineOfSightComponent.StartLineTrace` _lineofsight "TraceTypeQuery1" 60)
      (`LineOfSightComponent.StartBuildMesh` _lineofsight))))

(event `self.ReceiveUnpossessed`
  (params (OldController :type "Controller Object Reference"))
  (bind _ai_controller (`self.AI_Controller`))
  (bind _returnvalue (`AIBlueprintHelperLibrary.GetBlackboard` _ai_controller))
  (cast `/Game/Blueprints/BP_PlayerController` OldController)
  (`PaperFlipbookComponent.SetFlipbook` (`self.Parasite_Flipbook`) null)
  (`Controller.Possess` _ai_controller self)
  (`BlackboardComponent.SetValueAsBool` _returnvalue "is Stanned?" true)
  (`KismetSystemLibrary.Delay` 4.0)
  (`BlackboardComponent.SetValueAsBool` _returnvalue "is Stanned?" false))

(event `self.ReceiveBeginPlay`
  (`parent.ReceiveBeginPlay`)
  (if (`self.Protected_By_Mask?`)
    (`PaperFlipbookComponent.SetFlipbook` (`self.Parasite_Flipbook`) "/Game/Flipbooks/FB_Mask.FB_Mask")))

(event `self.ReceiveActorBeginOverlap`
  (params (OtherActor :type "Actor Object Reference"))
  (`parent.ReceiveActorBeginOverlap` OtherActor))

(event `self.ReceiveTick`
  (params (DeltaSeconds :type "Float (single-precision)"))
  (`parent.ReceiveTick` DeltaSeconds)
  (cast `/Game/Blueprints/BP_PlayerController` (`self.GetController`))
  (if (not (`/Game/Blueprints/BP_PlayerController.Paused?` (cast `/Game/Blueprints/BP_PlayerController` (`GameplayStatics.GetPlayerController` 0) :!pure true)))
    (`/Engine/EditorBlueprintResources/StandardMacros.DoOnce` false :!label _label
      (:`Completed`
        (bind _output_get (set `self.Health` (- (`self.Health`) 0.125)))
        (if (> _output_get 0.0)
          (`KismetSystemLibrary.Delay` 0.25)
          (goto _label :!via `Reset`)
          (else
            (`self.Death`)))))))

(event `EnhancedInput|/Game/Inputs/IA_Action`
  (params (ActionValue :type Boolean) (ElapsedSeconds :type "Float (double-precision)") (TriggeredSeconds :type "Float (double-precision)") (InputAction :type "InputAction Object Reference" :default "/Game/Inputs/IA_Action.IA_Action"))
  (bind _arrow_gun (`self.Arrow_Gun`))
  (:`Triggered`
    (bind _returnvalue (`|SpawnActorFromClass` "/Game/Blueprints/BP_Parasite.BP_Parasite_C" (`KismetMathLibrary.MakeTransform` (+ (`SceneComponent.K2_GetComponentLocation` _arrow_gun) (* (`SceneComponent.GetForwardVector` _arrow_gun) -10.0)) (struct :`Roll` 270.0)) "AdjustIfPossibleButDontSpawnIfColliding" "MultiplyWithRoot" null null))
    (`/Engine/EditorBlueprintResources/StandardMacros.IsValid` _returnvalue
      (:`Is Valid`
        (`Controller.Possess` (`self.GetController`) _returnvalue)
        (`self.Death`)))))

(fn `Debug_Show_Path`
  (bind _patrol_points (`self.Patrol_Points`))
  (bind _returnvalue (`KismetArrayLibrary.Array_LastIndex` _patrol_points))
  (for _index (range (+ _returnvalue 1))
    (`KismetSystemLibrary.DrawDebugLine` (`self.K2_GetActorLocation` (`|GetArrayItem` _patrol_points _index)) (`self.K2_GetActorLocation` (`|GetArrayItem` _patrol_points (mod (+ _index 1) (`KismetArrayLibrary.Array_Length` _patrol_points)))) (`KismetMathLibrary.LinearColorLerp` (struct :`R` 0.036493 :`G` 1.0 :`A` 1.0) (struct :`R` 1.0 :`G` 0.007579 :`A` 1.0) (/ (`KismetMathLibrary.Conv_IntToDouble` _index) (`KismetMathLibrary.Conv_IntToDouble` _returnvalue))) 30.0 10.0)))

(fn `UserConstructionScript`
  (`parent.UserConstructionScript`))