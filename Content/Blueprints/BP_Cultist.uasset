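; BP_Cultist is a controllable pawn that moves along its up and forward axes and fires bullets.
; Vertical and horizontal Enhanced Input actions feed AddMovementInput along those actor vectors.
; A looping timer started on BeginPlay spawns a scaled-down BP_Bullet at ArrowGun's transform, with the cultist as owner.
; Left mouse input spawns the same bullet separately, without setting an owner.
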(event `Shooting`
  (bind (_returnvalue_location _returnvalue_rotation) (`KismetMathLibrary.BreakTransform` (`SceneComponent.K2_GetComponentToWorld` (`self.Arrow_Gun`))))
  (`|SpawnActorFromClass` "/Game/Blueprints/BP_Bullet.BP_Bullet_C" (`KismetMathLibrary.MakeTransform` _returnvalue_location _returnvalue_rotation (0.25 0.25 0.25)) "Undefined" "MultiplyWithRoot" self null))

(event `self.ReceiveBeginPlay`
  (`KismetSystemLibrary.K2_SetTimerDelegate` (delegate `Shooting`) 1.0 true))

(event `self.ReceiveTick`
  (params (DeltaSeconds :type "Float (single-precision)")))

(event `EnhancedInput|/Game/Old_BP/IA_LeftMouse`
  (params (ActionValue :type Boolean) (ElapsedSeconds :type "Float (double-precision)") (TriggeredSeconds :type "Float (double-precision)") (InputAction :type "InputAction Object Reference" :default "/Game/Old_BP/IA_LeftMouse.IA_LeftMouse"))
  (bind (_returnvalue_location _returnvalue_rotation) (`KismetMathLibrary.BreakTransform` (`SceneComponent.K2_GetComponentToWorld` (`self.Arrow_Gun`))))
  (:`Triggered`
    (`|SpawnActorFromClass` "/Game/Blueprints/BP_Bullet.BP_Bullet_C" (`KismetMathLibrary.MakeTransform` _returnvalue_location _returnvalue_rotation (0.25 0.25 0.25)) "Undefined" "MultiplyWithRoot" null null)))

(event `EnhancedInput|/Game/Old_BP/IA_Vertical`
  (params (ActionValue :type "Float (double-precision)") (ElapsedSeconds :type "Float (double-precision)") (TriggeredSeconds :type "Float (double-precision)") (InputAction :type "InputAction Object Reference" :default "/Game/Old_BP/IA_Vertical.IA_Vertical"))
  (:`Triggered`
    (`self.AddMovementInput` (`self.GetActorUpVector`) ActionValue)))

(event `EnhancedInput|/Game/Old_BP/IA_Horizontal`
  (params (ActionValue :type "Float (double-precision)") (ElapsedSeconds :type "Float (double-precision)") (TriggeredSeconds :type "Float (double-precision)") (InputAction :type "InputAction Object Reference" :default "/Game/Old_BP/IA_Horizontal.IA_Horizontal"))
  (:`Triggered`
    (`self.AddMovementInput` (`self.GetActorForwardVector`) ActionValue)))

(fn `UserConstructionScript`)