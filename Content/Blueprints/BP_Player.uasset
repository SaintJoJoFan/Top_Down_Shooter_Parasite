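; BP_Player is a 2D Paper2D player character that runs left and right, jumps, and dies on overlapping a BP_Hurt.
; Enhanced Input drives movement and jumping, rotating the sprite to face travel direction.
; Tick picks idle or jump flipbooks from vertical velocity, while death plays its flipbook, then sets GameOver on BP_PlayerController.
; The construction script selects one of four PaperSprite images from NumberDrone.
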(event `self.ReceiveBeginPlay`
  (bind _asbp_player_controller (cast `/Game/Blueprints/BP_PlayerController` (`self.GetController`)))
  (`EnhancedInputSubsystemInterface.AddMappingContext` (pcsubsystem `EnhancedInputLocalPlayerSubsystem` _asbp_player_controller) "/Game/Blueprints/IMC_Default.IMC_Default" 0 (struct)))

(event `EnhancedInput|/Game/Blueprints/IA_Horizontal`
  (params (ActionValue :type "Float (double-precision)") (ElapsedSeconds :type "Float (double-precision)") (TriggeredSeconds :type "Float (double-precision)") (InputAction :type "InputAction Object Reference" :default "/Game/Blueprints/IA_Horizontal.IA_Horizontal"))
  (:`Triggered`
    (`self.Animation_Moving` ActionValue))
  (:`Completed`
    (`self.Animation_StopMoving`)))

(event `EnhancedInput|/Game/Blueprints/IA_Jump`
  (params (ActionValue :type Boolean) (ElapsedSeconds :type "Float (double-precision)") (TriggeredSeconds :type "Float (double-precision)") (InputAction :type "InputAction Object Reference" :default "/Game/Blueprints/IA_Jump.IA_Jump"))
  (:`Triggered`
    (`self.Jumping`)))

(event `self.ReceiveTick`
  (params (DeltaSeconds :type "Float (single-precision)"))
  (if (not (or (`self.isJumping?`) (`self.isDying`)))
    (`self.Animation_Jumping`)))

(event `self.ReceiveActorBeginOverlap`
  (params (OtherActor :type "Actor Object Reference"))
  (bind _sprite (`self.Sprite`))
  (if (not (`self.isDying`))
    (cast `/Game/Blueprints/BP_Hurt` OtherActor)
    (set `self.isDying` true)
    (`self.Animation_Death`)
    (`KismetSystemLibrary.Delay` (`PaperFlipbookComponent.GetFlipbookLength` _sprite))
    (`PaperFlipbookComponent.Stop` _sprite)
    (bind _asbp_player_controller (cast `/Game/Blueprints/BP_PlayerController` (`GameplayStatics.GetPlayerController` 0)))
    (set `/Game/Blueprints/BP_PlayerController.Game_Over` true _asbp_player_controller)))

(event `self.ReceiveUnpossessed`
  (params (OldController :type "Controller Object Reference"))
  (if (not (`self.isDying`))
    (`PaperFlipbookComponent.SetFlipbook` (`self.Sprite`) "/Game/Assets/FB_Idle.FB_Idle")))

(fn `Animation_Death`
  (`PaperFlipbookComponent.SetFlipbook` (`self.Sprite`) "/Game/Assets/FB_Player_Death.FB_Player_Death"))

(fn `Animation_Jumping`
  (bind (_returnvalue_x _returnvalue_y _returnvalue_z) (`KismetMathLibrary.BreakVector` (`self.GetVelocity`)))
  (bind _sprite (`self.Sprite`))
  (if (and (not (`self.isMoving`)) (== _returnvalue_z 0.0))
    (`PaperFlipbookComponent.SetLooping` _sprite true)
    (`PaperFlipbookComponent.Play` _sprite)
    (`PaperFlipbookComponent.SetFlipbook` _sprite "/Game/Assets/FB_Idle.FB_Idle")
    (elif (> _returnvalue_z 0.0)
      (`PaperFlipbookComponent.SetLooping` _sprite true)
      (`PaperFlipbookComponent.Play` _sprite)
      (`PaperFlipbookComponent.SetFlipbook` _sprite "/Game/Assets/Textures/Player_Sprites/FB_Jump_Begin.FB_Jump_Begin")
      (elif (< _returnvalue_z 0.0)
        (`PaperFlipbookComponent.SetLooping` _sprite true)
        (`PaperFlipbookComponent.Play` _sprite)
        (`PaperFlipbookComponent.SetFlipbook` _sprite "/Game/Assets/Textures/Player_Sprites/FB_Jump_Over.FB_Jump_Over")))))

(fn `Animation_Moving`
  (params (Action_Value :type "Float (double-precision)"))
  (if (not (`self.isDying`))
    (set `self.isMoving` true)
    (`self.AddMovementInput` (`self.GetActorForwardVector`) Action_Value)
    (if (> Action_Value 0.0)
      (`SceneComponent.K2_SetWorldRotation` :`self` (`self.Sprite`))
      (else
        (`SceneComponent.K2_SetWorldRotation` (`self.Sprite`) (struct :`Yaw` -180.0) false false)))
    (if (not (or (`self.isJumping?`) (`self.isDying`)))
      (`PaperFlipbookComponent.SetFlipbook` (`self.Sprite`) "/Game/Assets/FB_Run.FB_Run"))))

(fn `Animation_StopMoving`
  (if (not (or (`self.isJumping?`) (`self.isDying`)))
    (`PaperFlipbookComponent.SetFlipbook` (`self.Sprite`) "/Game/Assets/FB_Idle.FB_Idle")
    (set `self.isMoving` false)))

(fn `Jumping`
  (if (not (or (`self.isJumping?`) (`self.isDying`)))
    (set `self.isJumping?` true)
    (`self.Jump`)
    (set `self.isJumping?` false)))

(fn `UserConstructionScript`
  (switch `int` (`self.Number_Drone`)
    (:`1`
      (`PaperSpriteComponent.SetSprite` (`self.PaperSprite`) "/Game/Assets/Textures/Effects_Sprite/1_Sprite.1_Sprite"))
    (:`2`
      (`PaperSpriteComponent.SetSprite` (`self.PaperSprite`) "/Game/Assets/Textures/Effects_Sprite/2_Sprite.2_Sprite"))
    (:`3`
      (`PaperSpriteComponent.SetSprite` (`self.PaperSprite`) "/Game/Assets/Textures/Effects_Sprite/3_Sprite.3_Sprite"))
    (:`4`
      (`PaperSpriteComponent.SetSprite` (`self.PaperSprite`) "/Game/Assets/Textures/Effects_Sprite/4_Sprite.4_Sprite"))))