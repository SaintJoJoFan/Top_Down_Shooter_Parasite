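; Game instance that owns the game's save data, holding a WS_Save_Game object in SavedGameRef.
; On Init it loads the single hardcoded slot if one exists, otherwise creates a fresh save object in memory.
; SaveGame writes that object synchronously to the slot, while NewGame replaces it without writing to disk.
; Save, load and new-game events print debug messages; the soundtrack event is an empty stub.
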(event `Save Game`
  (`KismetSystemLibrary.PrintString` "Game saved")
  (`GameplayStatics.SaveGameToSlot` (`self.Saved_Game_Ref`) "stupid save"))

(event `Load Game`
  (`KismetSystemLibrary.PrintString` "Game loaded")
  (bind _returnvalue (`GameplayStatics.LoadGameFromSlot` "stupid save"))
  (bind _asws_save_game (cast `/Game/Blueprints/WS_Save_Game` _returnvalue))
  (set `self.Saved_Game_Ref` _asws_save_game))

(event `New Game`
  (`KismetSystemLibrary.PrintString` "New Game Save")
  (bind _returnvalue (`GameplayStatics.CreateSaveGameObject` "/Game/Blueprints/WS_Save_Game.WS_Save_Game_C"))
  (set `self.Saved_Game_Ref` _returnvalue))

(event `self.ReceiveInit`
  (bind _returnvalue (`GameplayStatics.DoesSaveGameExist` "stupid save"))
  (if _returnvalue
    (`self.Load Game`)
    (else
      (`self.New Game`))))

(event `Play Sountrack`)