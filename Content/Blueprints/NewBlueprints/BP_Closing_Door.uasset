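; BP_Closing_Door is a sliding door actor that closes or opens through its CloseDoor and OpenDoor events.
; Each event toggles the Box collision, on for closing and off for opening, and plays its own 2D door sound.
; Separate timelines lerp the Cube's relative Z in opposite directions, and each triggers a world camera shake at the door when finished.
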(event `/Game/Blueprints/NewBlueprints/BPI_Events_Shared_Between_Actors.Close Door`
  (`PrimitiveComponent.SetCollisionEnabled` (`self.Box`) "QueryAndPhysics")
  (`GameplayStatics.PlaySound2D` "/Game/Sounds/Door/Loud_Door_Close.Loud_Door_Close" 1.0 1.0 0.0 null null)
  (bind (_direction _newtrack_0) (`Timeline|Close` :!via `PlayFromStart`)
    (:`Update`
      (`SceneComponent.K2_SetRelativeLocation` (`self.Cube`) (`KismetMathLibrary.MakeVector` 0.0 0.0 (`KismetMathLibrary.Lerp` -50.0 50.0 _newtrack_0)) false false))
    (:`Finished`
      (`GameplayStatics.PlayWorldCameraShake` "/Game/Blueprints/NewBlueprints/BP_Door_Camera_Shake.BP_Door_Camera_Shake_C" (`self.K2_GetActorLocation`) 0.0 1000.0))))

(event `/Game/Blueprints/NewBlueprints/BPI_Events_Shared_Between_Actors.Open Door`
  (`PrimitiveComponent.SetCollisionEnabled` (`self.Box`) "NoCollision")
  (`GameplayStatics.PlaySound2D` "/Game/Sounds/Door/Lab_Door_Open.Lab_Door_Open" 1.0 1.0 0.0 null null)
  (bind (_direction _newtrack_0) (`Timeline|Timeline` :!via `PlayFromStart`)
    (:`Update`
      (`SceneComponent.K2_SetRelativeLocation` (`self.Cube`) (`KismetMathLibrary.MakeVector` 0.0 0.0 (`KismetMathLibrary.Lerp` 50.0 -50.0 _newtrack_0)) false false))
    (:`Finished`
      (`GameplayStatics.PlayWorldCameraShake` "/Game/Blueprints/NewBlueprints/BP_Door_Camera_Shake.BP_Door_Camera_Shake_C" (`self.K2_GetActorLocation`) 0.0 1000.0))))

(fn `UserConstructionScript`)