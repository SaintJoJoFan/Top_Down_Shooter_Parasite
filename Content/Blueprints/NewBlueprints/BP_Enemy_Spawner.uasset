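; Enemy spawner actor that places an Acolyte, Fanatic or Mage cultist, chosen by EnemyType, slightly above its location.
; Unless set to spawn instantly, it waits a short random delay, shows a TextRender pentagram as a warning, then hides it and spawns after a second random delay.
; Spawned enemies register with the tied enemy counter if valid.
; The construction script fixes the TextRender's world rotation.
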(event `/Game/Blueprints/NewBlueprints/BPI_Events_Shared_Between_Actors.Spawn_Enemy`
  (bind _enemy_counter_tied (`self.Enemy Counter Tied`))
  (bind _enemy_counter_tied_2 (`self.Enemy Counter Tied`))
  (bind _enemy_counter_tied_3 (`self.Enemy Counter Tied`))
  (bind _returnvalue (+ (`self.K2_GetActorLocation`) (0.0 0.0 50.0)))
  (if (`self.Spawn Instantly Without Warning`)
    (switch `/Game/Blueprints/NewBlueprints/Enemy_Type` (`self.Enemy_Type`) :!label _label
      (:`NewEnumerator0`
        (bind _returnvalue_2 (`|SpawnActorFromClass` "/Game/Blueprints/BP_Cultist_Acolyte.BP_Cultist_Acolyte_C" (`KismetMathLibrary.MakeTransform` _returnvalue) "Undefined" "MultiplyWithRoot" null null))
        (`/Engine/EditorBlueprintResources/StandardMacros.IsValid` _enemy_counter_tied
          (:`Is Valid`
            (`KismetArrayLibrary.Array_Add` (`/Game/Blueprints/NewBlueprints/BP_Wave_Enemy_Counter.Spawned Enemies` _enemy_counter_tied) _returnvalue_2))))
      (:`NewEnumerator1`
        (bind _returnvalue_3 (`|SpawnActorFromClass` "/Game/Blueprints/BP_Cultist_Fanatic.BP_Cultist_Fanatic_C" (`KismetMathLibrary.MakeTransform` _returnvalue) "Undefined" "MultiplyWithRoot" null null))
        (`/Engine/EditorBlueprintResources/StandardMacros.IsValid` _enemy_counter_tied_2
          (:`Is Valid`
            (`KismetArrayLibrary.Array_Add` (`/Game/Blueprints/NewBlueprints/BP_Wave_Enemy_Counter.Spawned Enemies` _enemy_counter_tied_2) _returnvalue_3))))
      (:`NewEnumerator2`
        (bind _returnvalue_4 (`|SpawnActorFromClass` "/Game/Blueprints/BP_Cultist_Mage.BP_Cultist_Mage_C" (`KismetMathLibrary.MakeTransform` _returnvalue) "Undefined" "MultiplyWithRoot" null null))
        (`/Engine/EditorBlueprintResources/StandardMacros.IsValid` _enemy_counter_tied_3
          (:`Is Valid`
            (`KismetArrayLibrary.Array_Add` (`/Game/Blueprints/NewBlueprints/BP_Wave_Enemy_Counter.Spawned Enemies` _enemy_counter_tied_3) _returnvalue_4)))))
    (else
      (`KismetSystemLibrary.K2_SetTimerDelegate` (delegate `Set Pentagramm`) (`KismetMathLibrary.RandomFloatInRange` 0.0 0.5)))))

(event `Set Pentagramm`
  (`SceneComponent.SetHiddenInGame` (`self.TextRender`) false false)
  (`KismetSystemLibrary.K2_SetTimerDelegate` (delegate `Spawn Enemy`) (`KismetMathLibrary.RandomFloatInRange` 0.75 1.25)))

(event `Spawn Enemy`
  (`SceneComponent.SetHiddenInGame` (`self.TextRender`) true false)
  (goto _label))

(fn `UserConstructionScript`
  (`SceneComponent.K2_SetWorldRotation` (`self.TextRender`) (`KismetMathLibrary.ComposeRotators` (struct) (struct :`Pitch` 90.0 :`Yaw` 90.0)) false false))