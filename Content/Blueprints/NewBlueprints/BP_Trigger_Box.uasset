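; BP_Trigger_Box is a one-shot trigger volume that fires scripted events when the player pawn overlaps its box.
; A DoOnce gate messages the listed enemies to spawn, starts an optional programmed cutscene, and messages doors to close.
; The actor-trigger messages and optional player-controller goal update are wired to both the door loop's body and its exit, so they repeat per door and once afterward.
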(event `self.Box.OnComponentBeginOverlap`
  (params (OverlappedComponent :type "PrimitiveComponent Object Reference") (OtherActor :type "Actor Object Reference") (OtherComp :type "PrimitiveComponent Object Reference") (OtherBodyIndex :type Integer) (bFromSweep :type Boolean) (SweepResult :type "HitResult Structure (by ref)"))
  (bind _progranned_cutscene_to_trigger (`self.Progranned Cutscene to Trigger`))
  (if (== OtherActor (`GameplayStatics.GetPlayerPawn` 0))
    (`/Engine/EditorBlueprintResources/StandardMacros.DoOnce` false
      (:`Completed`
        (for _array_element (`self.Enemies to Spawn`)
          (message `/Game/Blueprints/NewBlueprints/BPI_Events_Shared_Between_Actors.Spawn_Enemy` _array_element))
        (`/Engine/EditorBlueprintResources/StandardMacros.IsValid` _progranned_cutscene_to_trigger
          (:`Is Valid`
            (message `/Game/Blueprints/NewBlueprints/BPI_Events_Shared_Between_Actors.Start Programmed Cutscene` _progranned_cutscene_to_trigger))
          (:`Is Not Valid`
            _))
        (for _array_element_2 (`self.Door to Close`)
          (message `/Game/Blueprints/NewBlueprints/BPI_Events_Shared_Between_Actors.Close Door` _array_element_2)
          (for _array_element_3 (`self.Actors to Trigger`) :!label _label
            (message `/Game/Blueprints/NewBlueprints/BPI_Events_Shared_Between_Actors.Triggered` _array_element_3))
          (if (`self.Use Set Goal`)
            (bind _asbp_player_controller (cast `/Game/Blueprints/BP_PlayerController` (`GameplayStatics.GetPlayerController` 0)))
            (set `/Game/Blueprints/BP_PlayerController.Is Goal Visible` true _asbp_player_controller)
            (set `/Game/Blueprints/BP_PlayerController.Goal` (`self.Current Goal`) _asbp_player_controller)))
        (goto _label)))))

(fn `UserConstructionScript`)