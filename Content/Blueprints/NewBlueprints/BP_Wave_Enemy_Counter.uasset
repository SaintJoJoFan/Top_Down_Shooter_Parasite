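; Wave counter actor that tracks enemy deaths and triggers the next encounter events when a required group is cleared.
; On BeginPlay it registers itself on the SpawnedEnemiesNeededDead entries and optionally seeds counts for initial and spawned groups.
; EnemyDeath decrements the matching group's count.
; At zero, each group's own DoOnce runs shared actions: message spawners and doors, start an optional cutscene and optionally set the player controller's goal.
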(event `self.ReceiveBeginPlay`
  (`|ExecutionSequence`
    (:`then_0`
      (for _array_element (`self.Spawned Enemies Needed Dead`)
        (set `/Game/Blueprints/NewBlueprints/BP_Enemy_Spawner.Enemy Counter Tied` self _array_element)))
    (:`then_1`
      (`|ExecutionSequence`
        (:`then_0`
          (if (`self.Need All Initial Enemies Dead`)
            (set `self.Number of Initial Enemies Needed Dead` (`KismetArrayLibrary.Array_Length` (`self.Initial Enemies Needed Dead`)))))
        (:`then_1`
          (if (`self.Need All Spawned Enemies Dead`)
            (set `self.Number of Spawned Enemies Needed Dead` (`KismetArrayLibrary.Array_Length` (`self.Spawned Enemies Needed Dead`)))))))))

(event `/Game/Blueprints/NewBlueprints/BPI_Events_Shared_Between_Actors.Enemy_Death`
  (params (`Dead Enemy` :type "/Game/Blueprints/BP_Characters_Parent Object Reference"))
  (bind _cutscene (`self.Cutscene`))
  (if (`KismetArrayLibrary.Array_Contains` (`self.Initial Enemies Needed Dead`) `Dead Enemy`)
    (`/Engine/EditorBlueprintResources/StandardMacros.DecrementInt` (`self.Number of Initial Enemies Needed Dead`)
      (:`  `
        (if (<= (`self.Number of Initial Enemies Needed Dead`) 0)
          (`/Engine/EditorBlueprintResources/StandardMacros.DoOnce` false
            (:`Completed`
              (for _array_element (`self.Enemies To Spawn`) :!label _label
                (message `/Game/Blueprints/NewBlueprints/BPI_Events_Shared_Between_Actors.Spawn_Enemy` _array_element))
              (for _array_element_2 (`self.Doors To Open`)
                (message `/Game/Blueprints/NewBlueprints/BPI_Events_Shared_Between_Actors.Open Door` _array_element_2))
              (`/Engine/EditorBlueprintResources/StandardMacros.IsValid` _cutscene
                (:`Is Valid`
                  (message `/Game/Blueprints/NewBlueprints/BPI_Events_Shared_Between_Actors.Start Programmed Cutscene` _cutscene))
                (:`Is Not Valid`
                  _))
              (if (`self.Use Set Goal`)
                (bind _asbp_player_controller (cast `/Game/Blueprints/BP_PlayerController` (`GameplayStatics.GetPlayerController` 0)))
                (set `/Game/Blueprints/BP_PlayerController.Goal` (`self.Current Goal`) _asbp_player_controller)))))))
    (elif (`KismetArrayLibrary.Array_Contains` (`self.Spawned Enemies`) `Dead Enemy`)
      (`/Engine/EditorBlueprintResources/StandardMacros.DecrementInt` (`self.Number of Spawned Enemies Needed Dead`)
        (:`  `
          (if (<= (`self.Number of Spawned Enemies Needed Dead`) 0)
            (`/Engine/EditorBlueprintResources/StandardMacros.DoOnce` false
              (:`Completed`
                (goto _label)))))))))

(fn `UserConstructionScript`)