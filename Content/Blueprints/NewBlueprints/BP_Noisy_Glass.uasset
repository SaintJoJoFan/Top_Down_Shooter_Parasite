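; BP_Noisy_Glass is a patch of glass that shifts around the player and makes noise when stepped into.
; Each Tick, three planes are lerped away from a nearby player, within a short radius of their stored start positions, otherwise back toward them, with Z targeted at world zero.
; When the player enters the Box, it emits a tagged MakeNoise event and spawns a noise particle effect at the actor.
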(event `self.ReceiveBeginPlay`
  (`KismetArrayLibrary.Array_Add` (`self.Glass Massive`) (`self.Plane`))
  (`KismetArrayLibrary.Array_Add` (`self.Glass Massive`) (`self.Plane1`))
  (`KismetArrayLibrary.Array_Add` (`self.Glass Massive`) (`self.Plane2`))
  (for _array_element (`self.Glass Massive`)
    (`KismetArrayLibrary.Array_Add` (`self.Initial Locations`) (`SceneComponent.K2_GetComponentLocation` _array_element))))

(event `self.ReceiveTick`
  (params (DeltaSeconds :type "Float (single-precision)"))
  (bind (_returnvalue_x _returnvalue_y) (`KismetMathLibrary.BreakVector` (`self.K2_GetActorLocation` (`GameplayStatics.GetPlayerPawn` 0))))
  (bind _returnvalue (`KismetMathLibrary.MakeVector` _returnvalue_x _returnvalue_y))
  (for (_array_element _array_index) (`self.Initial Locations`)
    (bind _output (`|GetArrayItem` (`self.Glass Massive`) _array_index))
    (bind _returnvalue_2 (`KismetMathLibrary.MakeVector` (.x _array_element) (.y _array_element)))
    (bind _returnvalue_3 (- _returnvalue _returnvalue_2))
    (`SceneComponent.K2_SetWorldLocation` _output (`KismetMathLibrary.SelectVector` (`KismetMathLibrary.VLerp` (`SceneComponent.K2_GetComponentLocation` _output) (+ _returnvalue (* (`KismetMathLibrary.Normal` _returnvalue_3) -30.0)) 0.1) (`KismetMathLibrary.VLerp` (`SceneComponent.K2_GetComponentLocation` _output) _returnvalue_2 0.1) (and (< (`KismetMathLibrary.VSize` _returnvalue_3) 30.0) (< (`KismetMathLibrary.VSize` (- (`SceneComponent.K2_GetComponentLocation` (`|GetArrayItem` (`self.Glass Massive`) _array_index)) _returnvalue_2)) 30.0))) false false)))

(event `self.Box.OnComponentBeginOverlap`
  (params (OverlappedComponent :type "PrimitiveComponent Object Reference") (OtherActor :type "Actor Object Reference") (OtherComp :type "PrimitiveComponent Object Reference") (OtherBodyIndex :type Integer) (bFromSweep :type Boolean) (SweepResult :type "HitResult Structure (by ref)"))
  (bind _returnvalue_location (`KismetMathLibrary.BreakTransform` (`self.GetTransform`)))
  (if (== OtherActor (`GameplayStatics.GetPlayerPawn` 0))
    (`self.MakeNoise` 1.0 null _returnvalue_location 100.0 "noise")
    (`NiagaraFunctionLibrary.SpawnSystemAtLocation` "/Game/Particles/Particle_Noise.Particle_Noise" _returnvalue_location)))

(fn `UserConstructionScript`)