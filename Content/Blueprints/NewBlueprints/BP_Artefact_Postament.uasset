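; Artefact pedestal with a spinning sphere that the player takes through the Interract event, setting HasArtefact on BP_PlayerController.
; Taking it hides the sphere and prompt, then messages linked enemies to spawn, doors to close and an optional programmed cutscene to start.
; It also enables collision on linked triggerboxes.
; If the player already holds an artefact, the prompt shows a notice and a timer restores it.
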(event `self.ReceiveTick`
  (params (DeltaSeconds :type "Float (single-precision)"))
  (`SceneComponent.K2_AddLocalRotation` (`self.Sphere`) (struct :`Yaw` 1.0) false false))

(event `/Game/Blueprints/NewBlueprints/BPI_Events_Shared_Between_Actors.Interract`
  (bind _programmed_cutscene (`self.Programmed Cutscene`))
  (bind _asbp_player_controller (cast `/Game/Blueprints/BP_PlayerController` (`GameplayStatics.GetPlayerController` 0)))
  (if (`/Game/Blueprints/BP_PlayerController.Has Artefact` _asbp_player_controller)
    (`KismetSystemLibrary.K2_SetTimerDelegate` (delegate `Set Text Back`) 2.0)
    (`TextRenderComponent.K2_SetText` (`self.TextRender`) "You already have Artefact")
    (else
      (set `/Game/Blueprints/BP_PlayerController.Has Artefact` true _asbp_player_controller)
      (`SceneComponent.SetHiddenInGame` (`self.Sphere`) true false)
      (`SceneComponent.SetHiddenInGame` (`self.TextRender`) true false)
      (for _array_element (`self.Enemies To Spawn`)
        (message `/Game/Blueprints/NewBlueprints/BPI_Events_Shared_Between_Actors.Spawn_Enemy` _array_element))
      (for _array_element_2 (`self.Doors To Close`)
        (message `/Game/Blueprints/NewBlueprints/BPI_Events_Shared_Between_Actors.Close Door` _array_element_2))
      (`/Engine/EditorBlueprintResources/StandardMacros.IsValid` _programmed_cutscene
        (:`Is Valid`
          (message `/Game/Blueprints/NewBlueprints/BPI_Events_Shared_Between_Actors.Start Programmed Cutscene` _programmed_cutscene))
        (:`Is Not Valid`
          _))
      (for _array_element_3 (`self.Triggerboxes_To_Make_Valid`)
        (`PrimitiveComponent.SetCollisionEnabled` (`/Game/Blueprints/NewBlueprints/BP_Trigger_Box.Box` _array_element_3) "QueryAndPhysics")))))

(event `Set Text Back`
  (`TextRenderComponent.K2_SetText` (`self.TextRender`) "F to take Artefact"))

(fn `UserConstructionScript`)