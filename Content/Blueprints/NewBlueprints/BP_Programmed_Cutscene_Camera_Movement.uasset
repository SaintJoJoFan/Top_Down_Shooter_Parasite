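; Placeable actor that runs a timed, programmed cutscene camera through BP_Player_Camera_Manager.
; On BeginPlay it caches the first player's camera manager.
; StartProgrammedCutscene sets the manager's programmed-cutscene flag, passes this actor's location as the cutscene location, and starts a timer for Duration.
; When the timer fires, EndCutscene clears the flag and zeroes the location.
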(event `self.ReceiveBeginPlay`
  (bind _asbp_player_camera_manager (cast `/Game/Blueprints/BP_Player_Camera_Manager` (`PlayerController.PlayerCameraManager` (`GameplayStatics.GetPlayerController` 0))))
  (set `self.As BP Player Camera Manager` _asbp_player_camera_manager))

(event `/Game/Blueprints/NewBlueprints/BPI_Events_Shared_Between_Actors.Start Programmed Cutscene`
  (set `/Game/Blueprints/BP_Player_Camera_Manager.Is Using Programmed Cutscene` true (`self.As BP Player Camera Manager`))
  (set `/Game/Blueprints/BP_Player_Camera_Manager.Programmed Cutscene Location` (`self.K2_GetActorLocation`) (`self.As BP Player Camera Manager`))
  (`KismetSystemLibrary.K2_SetTimerDelegate` (delegate `End Cutscene`) (`self.Duration`)))

(event `End Cutscene`
  (set `/Game/Blueprints/BP_Player_Camera_Manager.Is Using Programmed Cutscene` false (`self.As BP Player Camera Manager`))
  (set `/Game/Blueprints/BP_Player_Camera_Manager.Programmed Cutscene Location` (0.0 0.0 0.0) (`self.As BP Player Camera Manager`)))

(fn `UserConstructionScript`)