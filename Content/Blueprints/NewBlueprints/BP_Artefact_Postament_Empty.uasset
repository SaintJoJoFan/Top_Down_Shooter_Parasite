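; An empty artefact pedestal that the player interacts with to place a carried artefact and open doors.
; Interract checks HasArtefact on BP_PlayerController; if set, it clears the flag, shows the sphere, hides the prompt, messages every DoorsToOpen entry and starts the optional ProgrammedCutscene.
; Without an artefact, the prompt shows a warning and a timer restores it.
; Tick continuously spins the sphere.
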(event `self.ReceiveTick`
  (params (DeltaSeconds :type "Float (single-precision)"))
  (`SceneComponent.K2_AddLocalRotation` (`self.Sphere`) (struct :`Yaw` 1.0) false false))

(event `self.Interract`
  (bind _programmed_cutscene (`self.Programmed Cutscene`))
  (bind _asbp_player_controller (cast `/Game/Blueprints/BP_PlayerController` (`GameplayStatics.GetPlayerController` 0)))
  (if (`/Game/Blueprints/BP_PlayerController.Has Artefact` _asbp_player_controller)
    (set `/Game/Blueprints/BP_PlayerController.Has Artefact` false _asbp_player_controller)
    (`SceneComponent.SetVisibility` (`self.Sphere`) true false)
    (`SceneComponent.SetHiddenInGame` (`self.TextRender`) true false)
    (for _array_element (`self.Doors To Open`)
      (message `/Game/Blueprints/NewBlueprints/BPI_Events_Shared_Between_Actors.Open Door` _array_element))
    (`/Engine/EditorBlueprintResources/StandardMacros.IsValid` _programmed_cutscene
      (:`Is Valid`
        (message `/Game/Blueprints/NewBlueprints/BPI_Events_Shared_Between_Actors.Start Programmed Cutscene` _programmed_cutscene)))
    (else
      (`KismetSystemLibrary.K2_SetTimerDelegate` (delegate `Set Text Back`) 2.0)
      (`TextRenderComponent.K2_SetText` (`self.TextRender`) "You don't have Artefact"))))

(event `Set Text Back`
  (`TextRenderComponent.K2_SetText` (`self.TextRender`) "F to paste \nArtefact"))

(fn `UserConstructionScript`)