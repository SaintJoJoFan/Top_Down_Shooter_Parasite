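; Base character for player-controlled and enemy bodies in a 2D-sprite shooter, with movement input, pistol and three-bullet shotgun fire, and velocity-driven flipbook animation.
; Shots flag bullets as enemy-owned by controller type and emit noise.
; Damage flashes red, granting players brief invulnerability.
; Death notifies wave counters, then drops a corpse for non-players or moves the player into a new parasite, whose own death sets game over.
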(event `Shoot_Pistol`
  (bind _returnvalue_location (`KismetMathLibrary.BreakTransform` (`self.GetTransform`)))
  (bind (_returnvalue_location_2 _returnvalue_rotation _returnvalue_scale) (`KismetMathLibrary.BreakTransform` (`SceneComponent.K2_GetComponentToWorld` (`self.Arrow_Bullet`))))
  ;[1 1 1] Shoot Pistol
  (`|SpawnActorFromClass` "/Game/Blueprints/BP_Bullet.BP_Bullet_C" (`KismetMathLibrary.MakeTransform` _returnvalue_location_2 _returnvalue_rotation _returnvalue_scale) "AlwaysSpawn" "MultiplyWithRoot" self (`.bSuccess` (cast `/Game/Blueprints/BP_Enemy_Controller` (`self.GetController`) :!pure true)) (`self.Bullet_Speed`) null 6.0 false null)
  (`GameplayStatics.PlaySound2D` "/Game/Sounds/SND_Pistol_Shot.SND_Pistol_Shot" 1.0 1.0 0.0 null null)
  (`self.MakeNoise` 1.0 null (0.0 0.0 0.0) 100.0 "noise")
  (`NiagaraFunctionLibrary.SpawnSystemAtLocation` "/Game/Particles/Particle_Noise.Particle_Noise" _returnvalue_location))

(event `Shoot Shotgun`
  (bind _returnvalue_location (`KismetMathLibrary.BreakTransform` (`self.GetTransform`)))
  (bind _bullet_speed (`self.Bullet_Speed`))
  (bind _bullet_damage (`self.Bullet_Damage`))
  (bind _returnvalue (`SceneComponent.K2_GetComponentToWorld` (`self.Arrow_Bullet`)))
  (bind (_asbp_enemy_controller _bsuccess) (cast `/Game/Blueprints/BP_Enemy_Controller` (`self.GetController`) :!pure true))
  ;[1 1 1] Shoot Shotgun
  (`|SpawnActorFromClass` "/Game/Blueprints/BP_Bullet.BP_Bullet_C" (`KismetMathLibrary.MakeTransform` (.location _returnvalue) (`KismetMathLibrary.MakeRotator` (.roll (.rotation _returnvalue)) (.pitch (.rotation _returnvalue)) (.yaw (.rotation _returnvalue))) (.scale _returnvalue)) "AlwaysSpawn" "MultiplyWithRoot" self _bsuccess _bullet_speed null _bullet_damage false null)
  (`|SpawnActorFromClass` "/Game/Blueprints/BP_Bullet.BP_Bullet_C" (`KismetMathLibrary.MakeTransform` (.location _returnvalue) (`KismetMathLibrary.MakeRotator` (.roll (.rotation _returnvalue)) (.pitch (.rotation _returnvalue)) (+ (.yaw (.rotation _returnvalue)) 15.0)) (.scale _returnvalue)) "AlwaysSpawn" "MultiplyWithRoot" self _bsuccess _bullet_speed null _bullet_damage false null)
  (`|SpawnActorFromClass` "/Game/Blueprints/BP_Bullet.BP_Bullet_C" (`KismetMathLibrary.MakeTransform` (.location _returnvalue) (`KismetMathLibrary.MakeRotator` (.roll (.rotation _returnvalue)) (.pitch (.rotation _returnvalue)) (+ (.yaw (.rotation _returnvalue)) -15.0)) (.scale _returnvalue)) "AlwaysSpawn" "MultiplyWithRoot" self _bsuccess _bullet_speed null _bullet_damage false null)
  (`GameplayStatics.PlaySound2D` "/Game/Sounds/SND_Shotgun_Shot.SND_Shotgun_Shot" 1.0 1.0 0.0 null null)
  (`self.MakeNoise` 1.0 null (0.0 0.0 0.0) 300.0 "noise")
  (`NiagaraFunctionLibrary.SpawnSystemAtLocation` "/Game/Particles/Particle_Noise.Particle_Noise" _returnvalue_location))

(event `EnhancedInput|/Game/Inputs/IA_RightMouse`
  (params (ActionValue :type Boolean) (ElapsedSeconds :type "Float (double-precision)") (TriggeredSeconds :type "Float (double-precision)") (InputAction :type "InputAction Object Reference" :default "/Game/Inputs/IA_RightMouse.IA_RightMouse"))
  (:`Started`
    (set `self.Focused?` true))
  (:`Completed`
    (set `self.Focused?` false)))

(event `EnhancedInput|/Game/Inputs/IA_Vertical`
  (params (ActionValue :type "Float (double-precision)") (ElapsedSeconds :type "Float (double-precision)") (TriggeredSeconds :type "Float (double-precision)") (InputAction :type "InputAction Object Reference" :default "/Game/Inputs/IA_Vertical.IA_Vertical"))
  (:`Triggered`
    (if (not (`self.Is Stunned`))
      (`self.AddMovementInput` (`self.GetActorUpVector`) ActionValue))))

(event `EnhancedInput|/Game/Inputs/IA_Horizontal`
  (params (ActionValue :type "Float (double-precision)") (ElapsedSeconds :type "Float (double-precision)") (TriggeredSeconds :type "Float (double-precision)") (InputAction :type "InputAction Object Reference" :default "/Game/Inputs/IA_Horizontal.IA_Horizontal"))
  (:`Triggered`
    (if (not (`self.Is Stunned`))
      (`self.AddMovementInput` (`self.GetActorForwardVector`) ActionValue))))

(event `self.ReceiveAnyDamage`
  (params (Damage :type "Float (single-precision)") (DamageType :type "DamageType Object Reference") (InstigatedBy :type "Controller Object Reference") (DamageCauser :type "Actor Object Reference"))
  (bind _sprite (`self.Sprite`))
  (bind _sprite_2 (`self.Sprite`))
  (`GameplayStatics.PlaySound2D` "/Game/Sounds/SND_Flesh_Hit.SND_Flesh_Hit" 1.0 1.0 0.0 null null)
  (bind _output_get (set `self.Health` (- (`self.Health`) Damage)))
  (if (<= _output_get 0.5)
    (cast `/Game/Blueprints/BP_Parasite` self
      (:`then`
        (bind _asbp_player_controller (cast `/Game/Blueprints/BP_PlayerController` (`self.GetController`)))
        (set `/Game/Blueprints/BP_PlayerController.Game_Over` true _asbp_player_controller))
      (:`CastFailed`
        (`self.Death`)))
    (else
      (cast `/Game/Blueprints/BP_PlayerController` (`self.GetController`)
        (:`then`
          (set `self.bCanBeDamaged` false)
          (`PaperFlipbookComponent.SetSpriteColor` _sprite_2 (struct :`R` 1.0 :`A` 1.0))
          (`KismetSystemLibrary.Delay` 0.5)
          (set `self.bCanBeDamaged` true)
          (`PaperFlipbookComponent.SetSpriteColor` _sprite_2 (struct :`R` 1.0 :`G` 1.0 :`B` 1.0 :`A` 1.0)))
        (:`CastFailed`
          (`PaperFlipbookComponent.SetSpriteColor` _sprite (struct :`R` 1.0 :`A` 1.0))
          (`KismetSystemLibrary.Delay` 0.1)
          (`PaperFlipbookComponent.SetSpriteColor` _sprite (struct :`R` 1.0 :`G` 1.0 :`B` 1.0 :`A` 1.0)))))))

(event `self.ReceiveBeginPlay`
  (bind _outactors (`GameplayStatics.GetAllActorsOfClass` "/Game/Blueprints/NewBlueprints/BP_Wave_Enemy_Counter.BP_Wave_Enemy_Counter_C"))
  (set `self.Wave Counters` _outactors))

(event `Death`
  (bind _returnvalue (`self.GetTransform`))
  (for _array_element (`self.Wave Counters`)
    (message `/Game/Blueprints/NewBlueprints/BPI_Events_Shared_Between_Actors.Enemy_Death` _array_element self))
  (`GameplayStatics.PlaySound2D` "/Game/Sounds/SND_Deathblow.SND_Deathblow" 1.0 1.0 0.0 null null)
  (cast `/Game/Blueprints/BP_PlayerController` (`self.GetController`)
    (:`then`
      (`PrimitiveComponent.SetCollisionEnabled` (`self.CapsuleComponent`) "NoCollision")
      (bind _returnvalue_2 (`|SpawnActorFromClass` "/Game/Blueprints/BP_Parasite.BP_Parasite_C" (`self.GetTransform`) "Undefined" "MultiplyWithRoot" null null))
      (`Controller.Possess` (`self.GetController`) _returnvalue_2)
      (`self.K2_DestroyActor`))
    (:`CastFailed`
      (`|SpawnActorFromClass` "/Game/Blueprints/BP_Dead_Body.BP_Dead_Body_C" (`KismetMathLibrary.MakeTransform` (`KismetMathLibrary.MakeVector` (.x (.location _returnvalue)) (.y (.location _returnvalue)) 10.0) (.rotation _returnvalue) (.scale _returnvalue)) "AdjustIfPossibleButAlwaysSpawn" "OverrideRootScale" null null)
      (`self.K2_DestroyActor`))))

(event `self.ReceiveHit`
  (params (MyComp :type "PrimitiveComponent Object Reference") (Other :type "Actor Object Reference") (OtherComp :type "PrimitiveComponent Object Reference") (bSelfMoved :type Boolean) (HitLocation :type "Vector Structure") (HitNormal :type "Vector Structure") (NormalImpulse :type "Vector Structure") (Hit :type "HitResult Structure (by ref)")))

(fn `Animation_Machine`
  (params (Character_Flipbook :type "PaperFlipbookComponent Object Reference") (Right_Flipbook :type "PaperFlipbook Object Reference") (Down_Flipbook :type "PaperFlipbook Object Reference") (Up_Flipbook :type "PaperFlipbook Object Reference") (Arrow_Bullet :type "ArrowComponent Object Reference") (Arrow_Gun :type "ArrowComponent Object Reference") (Gun_Flipbook :type "PaperFlipbookComponent Object Reference") (Idle_Right :type "PaperFlipbook Object Reference") (Idle_Down :type "PaperFlipbook Object Reference") (Idle_Up :type "PaperFlipbook Object Reference") (Arrow_Sprite_Gun :type "ArrowComponent Object Reference") (Arrow_All_Sprites :type "ArrowComponent Object Reference"))
  (bind (_returnvalue_x _returnvalue_y) (`KismetMathLibrary.BreakVector` (`self.GetVelocity`)))
  (bind (_relativelocation_x _relativelocation_y _relativelocation_z) (`KismetMathLibrary.BreakVector` (`SceneComponent.RelativeLocation` Arrow_Gun)))
  (`|ExecutionSequence`
    (:`then_0`
      (`/Engine/EditorBlueprintResources/StandardMacros.IsValid` Character_Flipbook
        (:`Is Valid`
          (`/Engine/EditorBlueprintResources/StandardMacros.IsValid` Right_Flipbook
            (:`Is Valid`
              (`/Engine/EditorBlueprintResources/StandardMacros.IsValid` Down_Flipbook
                (:`Is Valid`
                  (`/Engine/EditorBlueprintResources/StandardMacros.IsValid` Up_Flipbook
                    (:`Is Valid`
                      (`|ExecutionSequence`
                        (:`then_0`
                          (`SceneComponent.K2_SetWorldRotation` Character_Flipbook (`KismetMathLibrary.MakeRotator` (+ 270.0 30.0)) false false)
                          (`/Engine/EditorBlueprintResources/StandardMacros.IsValid` Arrow_All_Sprites
                            (:`Is Valid`
                              (cast `/Game/Blueprints/BP_PlayerController` (`self.GetController`))
                              (`SceneComponent.K2_SetWorldRotation` Arrow_All_Sprites (`KismetMathLibrary.MakeRotator` (+ 270.0 30.0)) false false))))
                        (:`then_1`
                          (if (< (`KismetMathLibrary.VSize` (`self.GetVelocity`)) 3.0)
                            (`PaperFlipbookComponent.SetFlipbook` Character_Flipbook (`self.Idle_Flipbook`))
                            (elif (> (`KismetMathLibrary.Abs` _returnvalue_x) (`KismetMathLibrary.Abs` _returnvalue_y))
                              (if (> _returnvalue_x 0.0)
                                (`PaperFlipbookComponent.SetFlipbook` Character_Flipbook Right_Flipbook)
                                (`SceneComponent.SetRelativeScale3D` Character_Flipbook (0.13 0.13 0.13))
                                (set `self.Idle_Flipbook` Idle_Right)
                                (else
                                  (`PaperFlipbookComponent.SetFlipbook` Character_Flipbook Right_Flipbook)
                                  (`SceneComponent.SetRelativeScale3D` Character_Flipbook (-0.13 0.13 0.13))
                                  (set `self.Idle_Flipbook` Idle_Right)))
                              (elif (> _returnvalue_y 0.0)
                                (`PaperFlipbookComponent.SetFlipbook` Character_Flipbook Down_Flipbook)
                                (set `self.Idle_Flipbook` Idle_Down)
                                (else
                                  (`PaperFlipbookComponent.SetFlipbook` Character_Flipbook Up_Flipbook)
                                  (set `self.Idle_Flipbook` Idle_Up))))))))))))))))
    (:`then_1`
      (`/Engine/EditorBlueprintResources/StandardMacros.IsValid` Arrow_Gun
        (:`Is Valid`
          (`/Engine/EditorBlueprintResources/StandardMacros.IsValid` Gun_Flipbook
            (:`Is Valid`
              (`/Engine/EditorBlueprintResources/StandardMacros.IsValid` Arrow_Sprite_Gun
                (:`Is Valid`
                  (`SceneComponent.K2_SetRelativeRotation` Arrow_Sprite_Gun (`SceneComponent.RelativeRotation` Arrow_Gun) false false)
                  (`SceneComponent.K2_SetRelativeLocation` Arrow_Gun (`KismetMathLibrary.MakeVector` _relativelocation_x 1.0 _relativelocation_z) false false))))))))))

(fn `Get Predicted_Position`
  (params (Prediction_Time :type "Float (double-precision)"))
  (returns (Predicted_Position :type "Vector Structure"))
  (return (+ (`self.K2_GetActorLocation`) (* (`self.GetVelocity`) Prediction_Time))))

(fn `UserConstructionScript`)