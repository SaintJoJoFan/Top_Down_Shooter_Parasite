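; BP_Vent is a destructible vent that reacts when a BP_Bullet overlaps it.
; On a hit it plays the Vent_Fall sound, sets VentDestroyed on its linked SpawnerToDeactivate if valid, then destroys itself.
; The construction script shows or hides the TutorialTip component through TipVisible.
; Logic to turn the tip toward the camera and bob it with a looping timeline is present but never runs.
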(event `self.ReceiveBeginPlay`)

(event `self.ReceiveActorBeginOverlap`
  (params (OtherActor :type "Actor Object Reference"))
  (bind _spawner_to_deactivate (`self.Spawner_To_Deactivate`))
  (cast `/Game/Blueprints/BP_Bullet` OtherActor)
  (`GameplayStatics.PlaySound2D` "/Game/Sounds/Vent/Vent_Fall.Vent_Fall" 1.0 1.0 0.0 null null)
  (`/Engine/EditorBlueprintResources/StandardMacros.IsValid` _spawner_to_deactivate
    (:`Is Valid`
      (set `/Game/Blueprints/NewBlueprints/BP_Spawn_If_Vent_Not_Destroyed.Vent_Destroyed` true _spawner_to_deactivate))
    (:`Is Not Valid`
      _))
  (`self.K2_DestroyActor`))

(event `self.ReceiveTick`
  (params (DeltaSeconds :type "Float (single-precision)")))

(fn `UserConstructionScript`
  (`SceneComponent.SetVisibility` (`self.Tutorial Tip`) (`self.Tip Visible`) false))