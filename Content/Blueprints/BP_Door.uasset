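; BP_Door is a level exit that loads LevelName on overlap.
; With IsGoalKill set, it waits until no BP_Cultist_Parent actors remain, then loads the level or, if IsFinalLevel, sets Victory on the overlapping character's BP_PlayerController; otherwise only the player pawn triggers it.
; BeginPlay caches the player's exit arrow and sprite, but the arrow-aiming and door-opening flipbook logic is disconnected and Tick is empty.
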(event `self.ReceiveBeginPlay`
  (bind _asbp_characters_parent (cast `/Game/Blueprints/BP_Characters_Parent` (`GameplayStatics.GetPlayerPawn` 0)))
  (set `self.Exit Arrow` (`/Game/Blueprints/BP_Characters_Parent.Exit_Arrow` _asbp_characters_parent))
  (set `self.Exit Sprite` (`/Game/Blueprints/BP_Characters_Parent.Exit_Sprite` _asbp_characters_parent)))

(event `self.ReceiveActorBeginOverlap`
  (params (OtherActor :type "Actor Object Reference"))
  (if (`self.is_Goal_Kill?`)
    (bind _outactors (`GameplayStatics.GetAllActorsOfClass` "/Game/Blueprints/BP_Cultist_Parent.BP_Cultist_Parent_C"))
    (if (<= (`KismetArrayLibrary.Array_Length` _outactors) 0)
      (if (`self.Is_Final_Level?`)
        (bind _asbp_characters_parent (cast `/Game/Blueprints/BP_Characters_Parent` OtherActor))
        (bind _asbp_player_controller (cast `/Game/Blueprints/BP_PlayerController` (`Pawn.GetController` _asbp_characters_parent)))
        (set `/Game/Blueprints/BP_PlayerController.Victory!` true _asbp_player_controller)
        (else
          (`GameplayStatics.OpenLevel` (`self.Level Name`)))))
    (elif (== (`GameplayStatics.GetPlayerPawn` 0) OtherActor)
      (`GameplayStatics.OpenLevel` (`self.Level Name`)))))

(event `self.ReceiveTick`
  (params (DeltaSeconds :type "Float (single-precision)")))

(fn `UserConstructionScript`)