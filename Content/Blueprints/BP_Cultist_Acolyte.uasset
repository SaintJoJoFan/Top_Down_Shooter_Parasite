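; Cultist acolyte character, playable or AI-controlled, that walks and shoots a pistol using flipbook sprites.
; On possession it sets walk speed and bullet speed by controller type, making the player faster than the enemy AI.
; Tick feeds directional walk, idle and gun flipbooks into the AnimationMachine.
; Left-mouse input makes noise and calls ShootPistol, throttled by a ReloadTime countdown that only advances while that input fires.
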(event `self.ReceiveBeginPlay`
  (`parent.ReceiveBeginPlay`)
  (set `self.Idle_Flipbook` "/Game/Flipbooks/FB_Idle_Down.FB_Idle_Down")
  (bind _output_get (set `self.Health` 12.0))
  (set `self.Health_Max` _output_get))

(event `self.ReceiveUnpossessed`
  (params (OldController :type "Controller Object Reference"))
  (`parent.ReceiveUnpossessed` OldController))

(event `self.ReceivePossessed`
  (params (NewController :type "Controller Object Reference"))
  (`parent.ReceivePossessed` NewController)
  (cast `/Game/Blueprints/BP_PlayerController` NewController
    (:`then`
      (set `CharacterMovementComponent.MaxWalkSpeed` 250.0 (`self.CharacterMovement`))
      (set `self.Bullet_Speed` 800.0))
    (:`CastFailed`
      (cast `/Game/Blueprints/BP_Enemy_Controller` NewController)
      (set `CharacterMovementComponent.MaxWalkSpeed` 200.0 (`self.CharacterMovement`))
      (set `self.Bullet_Speed` 600.0))))

(event `self.ReceiveTick`
  (params (DeltaSeconds :type "Float (single-precision)"))
  (`parent.ReceiveTick` DeltaSeconds)
  (`self.Animation_Machine` (`self.Sprite`) "/Game/Flipbooks/FB_Walk_Right.FB_Walk_Right" "/Game/Flipbooks/FB_Walk_Down.FB_Walk_Down" "/Game/Flipbooks/FB_Walk_Up.FB_Walk_Up" (`self.Arrow_Bullet`) (`self.Arrow_Gun`) (`self.Gun_FlipBook`) "/Game/Flipbooks/FB_Idle_Right.FB_Idle_Right" "/Game/Flipbooks/FB_Idle_Down.FB_Idle_Down" "/Game/Flipbooks/FB_Idle_Up.FB_Idle_Up"))

(event `EnhancedInput|/Game/Inputs/IA_LeftMouse`
  (params (ActionValue :type Boolean) (ElapsedSeconds :type "Float (double-precision)") (TriggeredSeconds :type "Float (double-precision)") (InputAction :type "InputAction Object Reference" :default "/Game/Inputs/IA_LeftMouse.IA_LeftMouse"))
  (:`Triggered`
    (`self.MakeNoise` 1.0 null (0.0 0.0 0.0) 600.0 "noise")
    (if (<= (`self.Reload_Time`) 0.0)
      (`self.Shoot_Pistol`)
      (set `self.Reload_Time` 0.05)
      (else
        (set `self.Reload_Time` (- (`self.Reload_Time`) (* (stale `self.ReceiveTick` DeltaSeconds) 200.0)))))))

(fn `UserConstructionScript`
  (`parent.UserConstructionScript`))