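; Pressure-plate button actor that holds a linked door open while the player stands on it.
; BeginPlay stores the resting location and a pressed location slightly below it.
; Overlap begin and end with BP_Player toggle the Pressed flag and set the Open flag on the DoorToOpen reference.
; Tick uses VInterpTo to ease the whole actor toward the pressed or resting location.
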(event `self.ReceiveBeginPlay`
  (bind _returnvalue (`self.K2_GetActorLocation`))
  (set `self.Location_Start` _returnvalue)
  (set `self.Location_Pressed` (+ _returnvalue (0.0 0.0 -7.0))))

(event `self.ReceiveActorBeginOverlap`
  (params (OtherActor :type "Actor Object Reference"))
  (cast `/Game/Blueprints/BP_Player` OtherActor)
  (set `self.Pressed` true)
  (set `/Game/Blueprints/BP_Door.Open` true (`self.Door_To_Open`)))

(event `self.ReceiveActorEndOverlap`
  (params (OtherActor :type "Actor Object Reference"))
  (cast `/Game/Blueprints/BP_Player` OtherActor)
  (set `self.Pressed` false)
  (set `/Game/Blueprints/BP_Door.Open` false (`self.Door_To_Open`)))

(event `self.ReceiveTick`
  (params (DeltaSeconds :type "Float (single-precision)"))
  (if (`self.Pressed`)
    (`self.K2_SetActorLocation` (`KismetMathLibrary.VInterpTo` (`self.K2_GetActorLocation`) (`self.Location_Pressed`) (`GameplayStatics.GetWorldDeltaSeconds`) 5.0))
    (else
      (`self.K2_SetActorLocation` (`KismetMathLibrary.VInterpTo` (`self.K2_GetActorLocation`) (`self.Location_Start`) (`GameplayStatics.GetWorldDeltaSeconds`) 5.0)))))

(fn `UserConstructionScript`)