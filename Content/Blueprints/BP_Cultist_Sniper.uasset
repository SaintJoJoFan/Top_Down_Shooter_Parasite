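; BP_Cultist_Sniper is a purple cultist sniper character that can be possessed by either the player or an enemy controller.
; Possession sets walk and bullet speed by controller type, with the player getting faster values.
; Tick feeds directional walk and idle flipbooks, gun flipbook and arrow components into the AnimationMachine call.
; Left-mouse input calls AimSniperGun through a DoOnce that resets after a short delay, limiting the fire rate.
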(event `self.ReceiveBeginPlay`
  (`parent.ReceiveBeginPlay`)
  (set `self.Idle_Flipbook` "/Game/Flipbooks/FB_Cultists/FB_Acolyte/FB_Purple_Idle_Down.FB_Purple_Idle_Down")
  (bind _output_get (set `self.Health` 12.0))
  (set `self.Health_Max` _output_get))

(event `self.ReceiveUnpossessed`
  (params (OldController :type "Controller Object Reference"))
  (`parent.ReceiveUnpossessed` OldController))

(event `self.ReceivePossessed`
  (params (NewController :type "Controller Object Reference"))
  (`parent.ReceivePossessed` NewController)
  (cast `/Game/Blueprints/BP_PlayerController` NewController
    (:`then`
      (set `CharacterMovementComponent.MaxWalkSpeed` 250.0 (`self.CharacterMovement`))
      (set `self.Bullet_Speed` 4000.0))
    (:`CastFailed`
      (cast `/Game/Blueprints/BP_Enemy_Controller` NewController)
      (set `CharacterMovementComponent.MaxWalkSpeed` 200.0 (`self.CharacterMovement`))
      (set `self.Bullet_Speed` 2000.0))))

(event `self.ReceiveTick`
  (params (DeltaSeconds :type "Float (single-precision)"))
  (`parent.ReceiveTick` DeltaSeconds)
  (`self.Animation Machine` (`self.Sprite`) "/Game/Flipbooks/FB_Cultists/FB_Acolyte/FB_Purple_Walk_Right.FB_Purple_Walk_Right" "/Game/Flipbooks/FB_Cultists/FB_Acolyte/FB_Purple_Walk_Left.FB_Purple_Walk_Left" "/Game/Flipbooks/FB_Cultists/FB_Acolyte/FB_Purple_Walk_Down.FB_Purple_Walk_Down" "/Game/Flipbooks/FB_Cultists/FB_Acolyte/FB_Purple_Walk_Up.FB_Purple_Walk_Up" (`self.Arrow_Bullet`) (`self.Arrow_Gun`) (`self.Gun_FlipBook`) "/Game/Flipbooks/FB_Cultists/FB_Acolyte/FB_Purple_Idle_Right.FB_Purple_Idle_Right" "/Game/Flipbooks/FB_Cultists/FB_Acolyte/FB_Purple_Idle_Left.FB_Purple_Idle_Left" "/Game/Flipbooks/FB_Cultists/FB_Acolyte/FB_Purple_Idle_Down.FB_Purple_Idle_Down" "/Game/Flipbooks/FB_Cultists/FB_Acolyte/FB_Purple_Idle_Up.FB_Purple_Idle_Up" (`self.Arrow_Sprite_Gun`) (`self.Arrow_Root`)))

(event `EnhancedInput|/Game/Inputs/IA_LeftMouse`
  (params (ActionValue :type Boolean) (ElapsedSeconds :type "Float (double-precision)") (TriggeredSeconds :type "Float (double-precision)") (InputAction :type "InputAction Object Reference" :default "/Game/Inputs/IA_LeftMouse.IA_LeftMouse"))
  (:`Triggered`
    (`/Engine/EditorBlueprintResources/StandardMacros.DoOnce` false :!label _label
      (:`Completed`
        (`self.Aim Sniper Gun`)
        (`KismetSystemLibrary.Delay` 0.5)
        (goto _label :!via `Reset`)))))

(fn `UserConstructionScript`
  (`parent.UserConstructionScript`))