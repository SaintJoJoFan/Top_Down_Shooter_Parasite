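; BP_Bullet is a projectile for player and enemy shots that moves forward each tick unless the player controller is paused.
; On overlap it damages only the opposing side, and player bullets also write the shooter into the enemy's blackboard as its target.
; Bullets ignore each other, except AntiBullet ones, which cancel opposing bullets.
; Impact or lifetime expiry spawns an explosion and particles, and emits AI noise before destroying the actor.
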(event `self.ReceiveBeginPlay`
  (`KismetSystemLibrary.Delay` 10.0)
  (`self.Self_Destroy`))

(event `self.ReceiveTick`
  (params (DeltaSeconds :type "Float (single-precision)"))
  (bind (_returnvalue_x _returnvalue_y _returnvalue_z) (`KismetMathLibrary.BreakVector` (* (`self.GetActorForwardVector`) (`self.Bullet_Speed`) DeltaSeconds)))
  ;[1 1 1] Paused?
  (bind _asbp_player_controller (cast `/Game/Blueprints/BP_PlayerController` (`GameplayStatics.GetPlayerController` 0)))
  (if (not (`/Game/Blueprints/BP_PlayerController.Paused?` _asbp_player_controller))
    (`self.K2_AddActorWorldOffset` (`KismetMathLibrary.MakeVector` _returnvalue_x _returnvalue_y _returnvalue_z))))

(event `self.ReceiveActorBeginOverlap`
  (params (OtherActor :type "Actor Object Reference"))
  (bind _returnvalue (`self.GetOwner`))
  (bind _source_actor (`self.Source_Actor`))
  (bind _damage (`self.Damage`))
  (bind _aspawn (cast `Pawn` OtherActor)
    (:`then`
      (if (`self.Is_Enemy_Bullet?`)
        (bind _returnvalue_2 (`Pawn.GetController` _aspawn))
        (cast `/Game/Blueprints/BP_PlayerController` _returnvalue_2)
        (bind _asbp_characters_parent (cast `/Game/Blueprints/BP_Characters_Parent` OtherActor))
        (`GameplayStatics.ApplyDamage` _asbp_characters_parent _damage null _returnvalue)
        (else
          (bind _asbp_enemy_controller (cast `/Game/Blueprints/BP_Enemy_Controller` _returnvalue_2))
          (bind _asbp_characters_parent_2 (cast `/Game/Blueprints/BP_Characters_Parent` OtherActor))
          (bind _returnvalue_3 (`AIBlueprintHelperLibrary.GetBlackboard` _asbp_enemy_controller))
          (`BlackboardComponent.SetValueAsObject` _returnvalue_3 "FollowTarget" (`self.Source_Actor`))
          (`BlackboardComponent.SetValueAsBool` _returnvalue_3 "Can See?" true)
          (`/Engine/EditorBlueprintResources/StandardMacros.IsValid` _source_actor
            (:`Is Valid`
              (`BlackboardComponent.SetValueAsVector` (`AIBlueprintHelperLibrary.GetBlackboard` _asbp_enemy_controller) "Target_Position" (`self.K2_GetActorLocation` _source_actor)))
            (:`Is Not Valid`
              _))
          (`GameplayStatics.ApplyDamage` _asbp_characters_parent_2 _damage null _returnvalue)))
      (`self.Self_Destroy`))
    (:`CastFailed`
      (if (`self.Anti-Bullet?`)
        (bind _asbp_bullet (cast `/Game/Blueprints/BP_Bullet` OtherActor))
        (if (not (== (`self.Is_Enemy_Bullet?`) (`/Game/Blueprints/BP_Bullet.Is_Enemy_Bullet?` _asbp_bullet)))
          (`self.Self_Destroy` _asbp_bullet)
          (`self.Self_Destroy`))
        (else
          (cast `/Game/Blueprints/BP_Bullet` OtherActor
            (:`CastFailed`
              (`self.Self_Destroy`))))))))

(event `Self_Destroy`
  (bind (_returnvalue_location _returnvalue_rotation) (`KismetMathLibrary.BreakTransform` (`self.GetTransform`)))
  (bind _returnvalue_location_2 (`KismetMathLibrary.BreakTransform` (`self.GetTransform`)))
  ;[1 1 1] Self Destroy
  (`|SpawnActorFromClass` "/Game/Blueprints/BP_Explosion.BP_Explosion_C" (`KismetMathLibrary.MakeTransform` _returnvalue_location _returnvalue_rotation (0.5 0.5 0.5)) "Undefined" "OverrideRootScale" null null)
  (`self.MakeNoise` 1.0 (cast `Pawn` (`self.Source_Actor`) :!pure true) (0.0 0.0 0.0) 300.0 "noise")
  (`NiagaraFunctionLibrary.SpawnSystemAtLocation` "/Game/Particles/Particle_Noise.Particle_Noise" _returnvalue_location_2)
  (`self.K2_DestroyActor`))

(fn `UserConstructionScript`)