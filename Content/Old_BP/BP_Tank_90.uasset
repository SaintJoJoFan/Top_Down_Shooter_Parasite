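; BP_Tank_90 is a flipbook-sprite tank that patrols on its own and fires BP_Bullet on a reload timer.
; Each Tick it moves forward and flips 180 degrees when line traces detect an obstacle ahead or no ground below its front.
; The countdown triggers a shot from ShootingArrow with a brief shoot animation.
; While the player overlaps ShootTrigger, patrol and firing pause and the player is launched upward, gated by a delayed DoOnce.
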(event `self.ReceiveActorBeginOverlap`
  (params (OtherActor :type "Actor Object Reference"))
  (`parent.ReceiveActorBeginOverlap` OtherActor))

(event `self.ReceiveTick`
  (params (DeltaSeconds :type "Float (single-precision)"))
  (bind _returnvalue (`self.K2_GetActorLocation`))
  (bind _returnvalue_2 (`GameplayStatics.GetPlayerPawn` 0))
  (bind (_returnvalue_location _returnvalue_rotation) (`KismetMathLibrary.BreakTransform` (`SceneComponent.K2_GetComponentToWorld` (`self.Shooting arrow`))))
  (bind _returnvalue_3 (+ (`self.K2_GetActorLocation`) (* (`self.GetActorForwardVector`) 20.0)))
  (`parent.ReceiveTick` DeltaSeconds)
  (if (`PrimitiveComponent.IsOverlappingActor` (`self.Shoot Trigger`) _returnvalue_2)
    (`/Engine/EditorBlueprintResources/StandardMacros.DoOnce` false :!label _label
      (:`Completed`
        (bind _asbp_player (cast `/Game/Old_BP/BP_Player` _returnvalue_2))
        (`self.LaunchCharacter` _asbp_player (* (`KismetMathLibrary.Vector_Up`) 400.0) false true)
        (`KismetSystemLibrary.Delay` 0.5)
        (goto _label :!via `Reset`)))
    (else
      (`|ExecutionSequence`
        (:`then_0`
          (bind (_outhit _returnvalue_4) (`KismetSystemLibrary.LineTraceSingle` _returnvalue (+ _returnvalue (* (`self.GetActorForwardVector`) 30.0)) "TraceTypeQuery1"))
          (if _returnvalue_4
            (`self.K2_AddActorWorldRotation` (struct :`Yaw` 180.0))))
        (:`then_1`
          (`self.K2_AddActorWorldOffset` (* (`self.GetActorForwardVector`) 30.0 DeltaSeconds)))
        (:`then_2`
          (bind (_outhit_2 _returnvalue_5) (`KismetSystemLibrary.LineTraceSingle` :`Start` _returnvalue_3 :`End` (+ _returnvalue_3 (0.0 0.0 -30.0)) :`TraceChannel` "TraceTypeQuery1" :`TraceColor` (struct :`R` 0.165146 :`G` 0.133324 :`B` 1.0 :`A` 1.0)))
          (if (not _returnvalue_5)
            (`self.K2_AddActorWorldRotation` (struct :`Yaw` 180.0))))
        (:`then_3`
          (set `self.Reload` (- (`self.Reload`) DeltaSeconds))
          (if (<= (`self.Reload`) 0.0)
            (`/Engine/EditorBlueprintResources/StandardMacros.DoOnce` false :!label _label_2
              (:`Completed`
                (`PaperFlipbookComponent.SetFlipbook` (`self.Sprite`) "/Game/Assets/FB_Tank_Shoot_90.FB_Tank_Shoot_90")
                (`|SpawnActorFromClass` "/Game/Blueprints/BP_Bullet.BP_Bullet_C" (`KismetMathLibrary.MakeTransform` _returnvalue_location _returnvalue_rotation) "AlwaysSpawn" "OverrideRootScale" null null)
                (`KismetSystemLibrary.Delay` 0.5)
                (`PaperFlipbookComponent.SetFlipbook` (`self.Sprite`) "/Game/Assets/FB_Tank_Run_90.FB_Tank_Run_90")
                (set `self.Reload` 1.5)
                (goto _label_2 :!via `Reset`)))))))))

(fn `UserConstructionScript`
  (`parent.UserConstructionScript`))