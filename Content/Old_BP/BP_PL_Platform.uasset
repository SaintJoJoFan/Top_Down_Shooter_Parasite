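; Possessable Paper2D platform character that moves, jumps and spawns a BP_Jump_Pad at its transform on BeginPlay, passing itself as the follow target.
; Animation functions swap idle, run and jump flipbooks from movement, vertical velocity and dying state.
; The moving function also applies forward-axis input and flips the sprite by rotation.
; Losing possession resets it to idle unless it is dying.
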(event `self.ReceiveBeginPlay`
  (`parent.ReceiveBeginPlay`)
  (`|SpawnActorFromClass` "/Game/Old_BP/BP_Jump_Pad.BP_Jump_Pad_C" (`self.GetTransform`) "Undefined" "MultiplyWithRoot" null self null))

(event `self.ReceiveActorBeginOverlap`
  (params (OtherActor :type "Actor Object Reference")))

(event `self.ReceiveTick`
  (params (DeltaSeconds :type "Float (single-precision)"))
  (`parent.ReceiveTick` DeltaSeconds))

(event `self.ReceiveUnpossessed`
  (params (OldController :type "Controller Object Reference"))
  (if (not (`self.isDying`))
    (`PaperFlipbookComponent.SetFlipbook` (`self.Sprite`) "/Game/Assets/FB_Platform_Idle.FB_Platform_Idle")))

(fn `Animation_Jumping`
  (bind (_returnvalue_x _returnvalue_y _returnvalue_z) (`KismetMathLibrary.BreakVector` (`self.GetVelocity`)))
  (bind _sprite (`self.Sprite`))
  (if (and (not (`self.isMoving`)) (== _returnvalue_z 0.0))
    (`PaperFlipbookComponent.SetLooping` _sprite true)
    (`PaperFlipbookComponent.Play` _sprite)
    (`PaperFlipbookComponent.SetFlipbook` _sprite "/Game/Assets/FB_Platform_Idle.FB_Platform_Idle")
    (elif (> _returnvalue_z 0.0)
      (`PaperFlipbookComponent.SetLooping` _sprite true)
      (`PaperFlipbookComponent.Play` _sprite)
      (`PaperFlipbookComponent.SetFlipbook` _sprite "/Game/Assets/FB_Platform_Jump.FB_Platform_Jump")
      (elif (< _returnvalue_z 0.0)
        (`PaperFlipbookComponent.SetLooping` _sprite true)
        (`PaperFlipbookComponent.Play` _sprite)
        (`PaperFlipbookComponent.SetFlipbook` _sprite "/Game/Assets/FB_Platform_Jump.FB_Platform_Jump")))))

(fn `Animation_Moving`
  (params (Action_Value :type "Float (double-precision)"))
  (if (not (`self.isDying`))
    (set `self.isMoving` true)
    (`self.AddMovementInput` (`self.GetActorForwardVector`) Action_Value)
    (if (> Action_Value 0.0)
      (`SceneComponent.K2_SetWorldRotation` (`self.Sprite`) (struct :`Yaw` -180.0) false false)
      (else
        (`SceneComponent.K2_SetWorldRotation` :`self` (`self.Sprite`))))
    (if (not (or (`self.isJumping?`) (`self.isDying`)))
      (`PaperFlipbookComponent.SetFlipbook` (`self.Sprite`) "/Game/Assets/FB_Platform_Run.FB_Platform_Run"))))

(fn `Animation_StopMoving`
  (if (not (or (`self.isJumping?`) (`self.isDying`)))
    (`PaperFlipbookComponent.SetFlipbook` (`self.Sprite`) "/Game/Assets/FB_Platform_Idle.FB_Platform_Idle")
    (set `self.isMoving` false)))

(fn `UserConstructionScript`
  (`parent.UserConstructionScript`))