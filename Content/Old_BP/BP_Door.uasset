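; BP_Door is a door actor that slides vertically down and back up based on an Open flag.
; BeginPlay caches the start location and an open target slightly below it.
; Tick moves the actor toward either target with VInterpTo, without sweep, giving an eased slide.
; Nothing in this Blueprint sets Open, and the overlap event is empty.
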(event `self.ReceiveBeginPlay`
  (bind _returnvalue (`self.K2_GetActorLocation`))
  (set `self.Location_Start` _returnvalue)
  (set `self.Location_Pressed` (+ _returnvalue (0.0 0.0 -32.0))))

(event `self.ReceiveTick`
  (params (DeltaSeconds :type "Float (single-precision)"))
  (if (`self.Open`)
    (`self.K2_SetActorLocation` (`KismetMathLibrary.VInterpTo` (`self.K2_GetActorLocation`) (`self.Location_Pressed`) (`GameplayStatics.GetWorldDeltaSeconds`) 5.0))
    (else
      (`self.K2_SetActorLocation` (`KismetMathLibrary.VInterpTo` (`self.K2_GetActorLocation`) (`self.Location_Start`) (`GameplayStatics.GetWorldDeltaSeconds`) 5.0)))))

(fn `UserConstructionScript`)