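; BP_Enemy is an enemy actor that reacts to overlaps with bullets and trigger boxes until it is dying.
; Bullets flagged FriendlyFier remove one Health, then explode via BP_Explosion and are destroyed.
; At zero Health the enemy sets IsDying, spawns its own explosion and destroys itself.
; Overlapping a TriggerBox destroys the enemy with no explosion, and Tick and BeginPlay are empty.
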(event `self.ReceiveBeginPlay`)

(event `self.ReceiveTick`
  (params (DeltaSeconds :type "Float (single-precision)")))

(event `self.ReceiveActorBeginOverlap`
  (params (OtherActor :type "Actor Object Reference"))
  (if (not (`self.isDying`))
    (bind _asbp_bullet (cast `/Game/Old_BP/BP_Bullet` OtherActor)
      (:`then`
        (if (`/Game/Old_BP/BP_Bullet.friendlyFier` _asbp_bullet)
          (`|ExecutionSequence`
            (:`then_0`
              (set `self.health` (- (`self.health`) 1))
              (if (<= (`self.health`) 0)
                (set `self.isDying` true)
                (`|SpawnActorFromClass` "/Game/Old_BP/BP_Explosion.BP_Explosion_C" (`self.GetTransform`) "Undefined" "OverrideRootScale" null null)
                (`self.K2_DestroyActor`)))
            (:`then_1`
              (`|SpawnActorFromClass` "/Game/Old_BP/BP_Explosion.BP_Explosion_C" (`self.GetTransform` _asbp_bullet) "Undefined" "OverrideRootScale" null null)
              (`self.K2_DestroyActor` _asbp_bullet)))))
      (:`CastFailed`
        (cast `TriggerBox` OtherActor)
        (`self.K2_DestroyActor`)))))

(fn `UserConstructionScript`)