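; BP_PL_Drone is a drone character that moves vertically through velocity-change impulses on its CharacterMovement.
; The Jumping function pushes it upward, and the IA_Down input event pushes it downward with equal strength.
; The animation functions for jumping, moving and stopping are empty, with a forward AddMovementInput left unconnected in the moving one.
; BeginPlay, Tick, overlap and unpossess events do nothing.
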(event `self.ReceiveActorBeginOverlap`
  (params (OtherActor :type "Actor Object Reference")))

(event `self.ReceiveUnpossessed`
  (params (OldController :type "Controller Object Reference")))

(event `EnhancedInput|/Game/Old_BP/IA_Down`
  (params (ActionValue :type Boolean) (ElapsedSeconds :type "Float (double-precision)") (TriggeredSeconds :type "Float (double-precision)") (InputAction :type "InputAction Object Reference" :default "/Game/Old_BP/IA_Down.IA_Down"))
  (:`Triggered`
    (`CharacterMovementComponent.AddImpulse` (`self.CharacterMovement`) (* (`KismetMathLibrary.Vector_Down`) 40.0) true)))

(fn `Animation_Jumping`)

(fn `Animation_Moving`
  (params (Action_Value :type "Float (double-precision)")))

(fn `Animation_StopMoving`)

(fn `Jumping`
  (`CharacterMovementComponent.AddImpulse` (`self.CharacterMovement`) (* (`KismetMathLibrary.Vector_Up`) 40.0) true))

(fn `UserConstructionScript`
  (`parent.UserConstructionScript`))