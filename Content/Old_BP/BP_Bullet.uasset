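; BP_Bullet is a projectile actor that flies straight along its forward vector and spawns a BP_Explosion on impact.
; Each Tick, unless BP_PlayerController is paused, it line-traces a short distance ahead, ignoring the player pawn, and either explodes or moves forward at constant speed.
; A BeginPlay delay also explodes and destroys it after a fixed lifetime, independent of the pause check.
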(event `self.ReceiveBeginPlay`
  (`KismetSystemLibrary.Delay` 10.0)
  (`|SpawnActorFromClass` "/Game/Old_BP/BP_Explosion.BP_Explosion_C" (`self.GetTransform`) "Undefined" "OverrideRootScale" null null)
  (`self.K2_DestroyActor`))

(event `self.ReceiveTick`
  (params (DeltaSeconds :type "Float (single-precision)"))
  (bind _returnvalue (`self.K2_GetActorLocation`))
  (bind (_returnvalue_x _returnvalue_y _returnvalue_z) (`KismetMathLibrary.BreakVector` (* (`self.GetActorForwardVector`) 500.0 DeltaSeconds)))
  (bind _asbp_player_controller (cast `/Game/Blueprints/BP_PlayerController` (`GameplayStatics.GetPlayerController` 0)))
  (if (not (`/Game/Blueprints/BP_PlayerController.Paused?` _asbp_player_controller))
    (bind (_outhit _returnvalue_2) (`KismetSystemLibrary.LineTraceSingle` _returnvalue (+ _returnvalue (* (`self.GetActorForwardVector`) 20.0)) "TraceTypeQuery1" false (`|MakeArray` (`GameplayStatics.GetPlayerPawn` 0) :!type "Actor Object Reference")))
    (if _returnvalue_2
      (`|SpawnActorFromClass` "/Game/Old_BP/BP_Explosion.BP_Explosion_C" (`self.GetTransform`) "Undefined" "OverrideRootScale" null null)
      (`self.K2_DestroyActor`)
      (else
        (`self.K2_AddActorWorldOffset` (`KismetMathLibrary.MakeVector` _returnvalue_x _returnvalue_y _returnvalue_z))))))

(fn `UserConstructionScript`)